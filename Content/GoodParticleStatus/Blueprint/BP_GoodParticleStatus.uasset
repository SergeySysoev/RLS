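; Component that attaches status particle effects (buffs, head icons, shields, debuffs, ground effects) to its owning Character's mesh.
; GoodParticleStatusUpdate, optionally run on BeginPlay, maps EffectsStyle to scaled emitters at hand, head, body or root points.
; Buffs add a root power-up burst; Selection, Frozen and Chill add a root emitter.
; Only None/Clear destroys emitters tracked in NowParticle; other styles overwrite that list, and the power-up is untracked.
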(event Custom|GoodParticleStatus%20Update
  (bind _particle_size (Variables|GoodParticleStatusSettingInput|GetParticle%20Size))
  (bind _returnvalue (Math|Conversions|ToVector(Float) _particle_size))
  ;[1 1 1] Custom Event
  (switch Utilities|FlowControl|Switch|SwitchonEnum_GoodParticleStatus (Variables|GoodParticleStatusSettingInput|GetEffects%20Style)
    (:NewEnumerator2
      ;[1 1 1] Clear
      (for _array_element (Variables|Don'ttouchme!!|GetNow%20Particle)
        (Utilities|IsValid _array_element
          (:Is%20Valid
            (Components|DestroyComponent _array_element))))
      (Utilities|Array|Clear (Variables|Don'ttouchme!!|GetNow%20Particle)))
    (:NewEnumerator16
      ;[1 1 1] Buff
      (Variables|Don'ttouchme!!|SetTemp%20Particle (Variables|GoodParticleStatusParticleSetting|GetBuff%20:%20EnergyLightning))
      (Variables|Don'ttouchme!!|SetTemp%20Size (Variables|GoodParticleStatusSettingInput|GetParticle%20Size) :!label _label)
      (bind _meshcomponent (CallFunction|FindMesh))
      (bind _returnvalue_2 (Effects|SpawnEmitterAttached (Variables|Don'ttouchme!!|GetTemp%20Particle) _meshcomponent (Variables|GoodParticleStatusSettingInput|GetRight%20Hand%20Point%20Name) "0, 0, 0" "0, 0, 0" (Math|Conversions|ToVector(Float) (Variables|Don'ttouchme!!|GetTemp%20Size))))
      (bind _returnvalue_3 (Effects|SpawnEmitterAttached (Variables|Don'ttouchme!!|GetTemp%20Particle) _meshcomponent (Variables|GoodParticleStatusSettingInput|GetLeft%20Hand%20Point%20Name) "0, 0, 0" "0, 0, 0" (Math|Conversions|ToVector(Float) (Variables|Don'ttouchme!!|GetTemp%20Size))))
      (Variables|Don'ttouchme!!|SetNow%20Particle (Utilities|Array|MakeArray _returnvalue_3 _returnvalue_2))
      ;[1 1 1] Add Power up
      (bind _meshcomponent_2 (CallFunction|FindMesh))
      (Effects|SpawnEmitterAttached "/Game/GoodParticleStatus/Particles/Buff_Status/PS_GPS_Buff_PowerUp.PS_GPS_Buff_PowerUp" _meshcomponent_2 (Variables|GoodParticleStatusSettingInput|GetRoot%20Point%20Name) "0, 0, 0" "0, 0, 0" (Math|Conversions|ToVector(Float) (Variables|Don'ttouchme!!|GetTemp%20Size))))
    (:NewEnumerator3
      (Variables|Don'ttouchme!!|SetTemp%20Particle (Variables|GoodParticleStatusParticleSetting|GetBuff%20:%20Fire))
      (goto _label))
    (:NewEnumerator15
      (Variables|Don'ttouchme!!|SetTemp%20Particle (Variables|GoodParticleStatusParticleSetting|GetBuff%20:%20Nebula))
      (goto _label))
    (:NewEnumerator1
      (Variables|Don'ttouchme!!|SetTemp%20Particle (Variables|GoodParticleStatusParticleSetting|GetBuff%20:%20Trail%20Ice))
      (goto _label))
    (:NewEnumerator8
      (Variables|Don'ttouchme!!|SetTemp%20Particle (Variables|GoodParticleStatusParticleSetting|GetBuff%20:%20Trail%20Poison))
      (goto _label))
    (:NewEnumerator0
      (Variables|Don'ttouchme!!|SetTemp%20Particle (Variables|GoodParticleStatusParticleSetting|GetBuff%20:%20Trail%20Soft))
      (goto _label))
    (:NewEnumerator17
      (Variables|Don'ttouchme!!|SetTemp%20Particle (Variables|GoodParticleStatusParticleSetting|GetBuff%20:%20Trail%20Sparks))
      (goto _label))
    (:NewEnumerator18
      (Variables|Don'ttouchme!!|SetTemp%20Particle (Variables|GoodParticleStatusParticleSetting|GetBuff%20:%20Trail%20Spirit%20Wave))
      (goto _label))
    (:NewEnumerator25
      (Variables|Don'ttouchme!!|SetTemp%20Particle (Variables|GoodParticleStatusParticleSetting|GetBuff%20:%20DarkFlame))
      (goto _label))
    (:NewEnumerator6
      ;[1 1 1] Head
      (Variables|Don'ttouchme!!|SetTemp%20Particle (Variables|GoodParticleStatusParticleSetting|GetHead%20:%20Chaos))
      (Variables|Don'ttouchme!!|SetTemp%20Point%20Name (Variables|GoodParticleStatusSettingInput|GetAbove%20The%20Head%20Point%20Name) :!label _label_2)
      (Variables|Don'ttouchme!!|SetTemp%20Size (Variables|GoodParticleStatusSettingInput|GetParticle%20Size) :!label _label_3)
      (bind _meshcomponent_3 (CallFunction|FindMesh))
      (bind _returnvalue_4 (Effects|SpawnEmitterAttached (Variables|Don'ttouchme!!|GetTemp%20Particle) _meshcomponent_3 (Variables|Don'ttouchme!!|GetTemp%20Point%20Name) "0, 0, 0" "0, 0, 0" (Math|Conversions|ToVector(Float) (Variables|Don'ttouchme!!|GetTemp%20Size))))
      (Variables|Don'ttouchme!!|SetNow%20Particle (Utilities|Array|MakeArray _returnvalue_4)))
    (:NewEnumerator27
      (Variables|Don'ttouchme!!|SetTemp%20Particle (Variables|GoodParticleStatusParticleSetting|GetHead%20:%20Eagle%20Vision))
      (goto _label_2))
    (:NewEnumerator21
      (Variables|Don'ttouchme!!|SetTemp%20Particle (Variables|GoodParticleStatusParticleSetting|GetHead%20:%20Evil))
      (goto _label_2))
    (:NewEnumerator22
      (Variables|Don'ttouchme!!|SetTemp%20Particle (Variables|GoodParticleStatusParticleSetting|GetHead%20:%20Exclamation%20Mark))
      (goto _label_2))
    (:NewEnumerator26
      (Variables|Don'ttouchme!!|SetTemp%20Particle (Variables|GoodParticleStatusParticleSetting|GetHead%20:Heart))
      (goto _label_2))
    (:NewEnumerator23
      (Variables|Don'ttouchme!!|SetTemp%20Particle (Variables|GoodParticleStatusParticleSetting|GetHead%20:QuestionMark))
      (goto _label_2))
    (:NewEnumerator24
      (Variables|Don'ttouchme!!|SetTemp%20Particle (Variables|GoodParticleStatusParticleSetting|GetHead%20:%20Selection))
      (bind _meshcomponent_4 (CallFunction|FindMesh))
      (bind _returnvalue_5 (Effects|SpawnEmitterAttached (Variables|Don'ttouchme!!|GetTemp%20Particle) _meshcomponent_4 (Variables|GoodParticleStatusSettingInput|GetAbove%20The%20Head%20Point%20Name) "0, 0, 0" "0, 0, 0" (Math|Conversions|ToVector(Float) (Variables|Don'ttouchme!!|GetTemp%20Size))))
      (bind _returnvalue_6 (Effects|SpawnEmitterAttached "/Game/GoodParticleStatus/Particles/Head_Status/PS_GPS_Selection_02.PS_GPS_Selection_02" _meshcomponent_4 (Variables|GoodParticleStatusSettingInput|GetRoot%20Point%20Name) "0, 0, 0" "0, 0, 0" (Math|Conversions|ToVector(Float) (Variables|Don'ttouchme!!|GetTemp%20Size))))
      (Variables|Don'ttouchme!!|SetNow%20Particle (Utilities|Array|MakeArray _returnvalue_6 _returnvalue_5)))
    (:NewEnumerator7
      (Variables|Don'ttouchme!!|SetTemp%20Particle (Variables|GoodParticleStatusParticleSetting|GetHead%20:%20Slience))
      (goto _label_2))
    (:NewEnumerator5
      (Variables|Don'ttouchme!!|SetTemp%20Particle (Variables|GoodParticleStatusParticleSetting|GetHead%20:%20Sleep%20))
      (goto _label_2))
    (:NewEnumerator4
      (Variables|Don'ttouchme!!|SetTemp%20Particle (Variables|GoodParticleStatusParticleSetting|GetHead%20:%20Stun%20))
      (goto _label_2))
    (:NewEnumerator19
      (Variables|Don'ttouchme!!|SetTemp%20Particle (Variables|GoodParticleStatusParticleSetting|GetHead%20:Unlucky%20))
      (goto _label_2))
    (:NewEnumerator14
      ;[1 1 1] Status
      (Variables|Don'ttouchme!!|SetTemp%20Particle (Variables|GoodParticleStatusParticleSetting|GetStatus%20:%20Shield%20Fire))
      (Variables|Don'ttouchme!!|SetTemp%20Point%20Name (Variables|GoodParticleStatusSettingInput|GetBody%20Center%20Point%20Name) :!label _label_4)
      (goto _label_3))
    (:NewEnumerator20
      (Variables|Don'ttouchme!!|SetTemp%20Particle (Variables|GoodParticleStatusParticleSetting|GetStatus%20:%20Shield%20HiTech))
      (goto _label_4))
    (:NewEnumerator13
      (Variables|Don'ttouchme!!|SetTemp%20Particle (Variables|GoodParticleStatusParticleSetting|GetStatus%20:%20Shield%20Water))
      (goto _label_4))
    (:NewEnumerator12
      (Variables|Don'ttouchme!!|SetTemp%20Particle (Variables|GoodParticleStatusParticleSetting|GetStatus%20:%20Shield%20))
      (goto _label_4))
    (:NewEnumerator10
      (Variables|Don'ttouchme!!|SetTemp%20Particle (Variables|GoodParticleStatusParticleSetting|GetDebuff%20Status%20:%20Burning))
      (goto _label_4))
    (:NewEnumerator11
      ;[1 1 1] Root : Status
      (Variables|Don'ttouchme!!|SetTemp%20Size (Variables|GoodParticleStatusSettingInput|GetParticle%20Size))
      (bind _meshcomponent_5 (CallFunction|FindMesh))
      (bind _returnvalue_7 (Effects|SpawnEmitterAttached (Variables|GoodParticleStatusParticleSetting|GetDeBuff%20:%20Frozen%20Particle) _meshcomponent_5 (Variables|GoodParticleStatusSettingInput|GetBody%20Center%20Point%20Name) "0, 0, 0" "0, 0, 0" (Math|Conversions|ToVector(Float) (Variables|Don'ttouchme!!|GetTemp%20Size))))
      (bind _returnvalue_8 (Effects|SpawnEmitterAttached "/Game/GoodParticleStatus/Particles/Status/Debuff_Status/PS_GPS_Frozen_02.PS_GPS_Frozen_02" _meshcomponent_5 (Variables|GoodParticleStatusSettingInput|GetRoot%20Point%20Name) "0, 0, 0" "0, 0, 0" (Math|Conversions|ToVector(Float) (Variables|Don'ttouchme!!|GetTemp%20Size))))
      (Variables|Don'ttouchme!!|SetNow%20Particle (Utilities|Array|MakeArray _returnvalue_8 _returnvalue_7)))
    (:NewEnumerator32
      (Variables|Don'ttouchme!!|SetTemp%20Particle (Variables|GoodParticleStatusParticleSetting|GetStatus%20:%20Backfire))
      (goto _label_4))
    (:NewEnumerator33
      (Variables|Don'ttouchme!!|SetTemp%20Particle (Variables|GoodParticleStatusParticleSetting|GetDebuff%20Status%20:%20Tar))
      (Variables|Don'ttouchme!!|SetTemp%20Point%20Name (Variables|GoodParticleStatusSettingInput|GetRoot%20Point%20Name))
      (goto _label_3))
    (:NewEnumerator34
      (Variables|Don'ttouchme!!|SetTemp%20Particle (Variables|GoodParticleStatusParticleSetting|GetDebuff%20Status%20:%20Chill))
      (bind _meshcomponent_6 (CallFunction|FindMesh))
      (bind _returnvalue_9 (Effects|SpawnEmitterAttached (Variables|Don'ttouchme!!|GetTemp%20Particle) _meshcomponent_6 (Variables|GoodParticleStatusSettingInput|GetBody%20Center%20Point%20Name) "0, 0, 0" "0, 0, 0" _returnvalue))
      (bind _returnvalue_10 (Effects|SpawnEmitterAttached "/Game/GoodParticleStatus/Particles/Status/Debuff_Status/PS_GPS_Chill_02.PS_GPS_Chill_02" _meshcomponent_6 (Variables|GoodParticleStatusSettingInput|GetRoot%20Point%20Name) "0, 0, 0" "0, 0, 0" _returnvalue))
      (Variables|Don'ttouchme!!|SetNow%20Particle (Utilities|Array|MakeArray _returnvalue_10 _returnvalue_9)))
    (:NewEnumerator28
      (Variables|Don'ttouchme!!|SetTemp%20Particle (Variables|GoodParticleStatusParticleSetting|GetRoot%20:%20Lake))
      (Variables|Don'ttouchme!!|SetTemp%20Point%20Name (Variables|GoodParticleStatusSettingInput|GetRoot%20Point%20Name) :!label _label_5)
      (goto _label_3))
    (:NewEnumerator29
      (Variables|Don'ttouchme!!|SetTemp%20Particle (Variables|GoodParticleStatusParticleSetting|GetRoot%20:%20Lava))
      (goto _label_5))
    (:NewEnumerator30
      (Variables|Don'ttouchme!!|SetTemp%20Particle (Variables|GoodParticleStatusParticleSetting|GetRoot%20:%20Snow))
      (goto _label_5))
    (:NewEnumerator31
      (Variables|Don'ttouchme!!|SetTemp%20Particle (Variables|GoodParticleStatusParticleSetting|GetRoot%20:%20Swamp))
      (goto _label_5))))

(event EventBeginPlay
  (bind _particle_size (Variables|GoodParticleStatusSettingInput|GetParticle%20Size))
  (bind _returnvalue (Math|Conversions|ToVector(Float) _particle_size))
  ;[1 1 1] check Begin Play
  (if (Variables|GoodParticleStatusSettingInput|GetbUse%20Event%20Begin%20Play)
    (switch Utilities|FlowControl|Switch|SwitchonEnum_GoodParticleStatus (Variables|GoodParticleStatusSettingInput|GetEffects%20Style)
      (:NewEnumerator2
        ;[1 1 1] Clear
        (for _array_element (Variables|Don'ttouchme!!|GetNow%20Particle)
          (Utilities|IsValid _array_element
            (:Is%20Valid
              (Components|DestroyComponent _array_element))))
        (Utilities|Array|Clear (Variables|Don'ttouchme!!|GetNow%20Particle)))
      (:NewEnumerator16
        ;[1 1 1] Buff
        (Variables|Don'ttouchme!!|SetTemp%20Particle (Variables|GoodParticleStatusParticleSetting|GetBuff%20:%20EnergyLightning))
        (Variables|Don'ttouchme!!|SetTemp%20Size (Variables|GoodParticleStatusSettingInput|GetParticle%20Size) :!label _label)
        (bind _meshcomponent (CallFunction|FindMesh))
        (bind _returnvalue_2 (Effects|SpawnEmitterAttached (Variables|Don'ttouchme!!|GetTemp%20Particle) _meshcomponent (Variables|GoodParticleStatusSettingInput|GetRight%20Hand%20Point%20Name) "0, 0, 0" "0, 0, 0" (Math|Conversions|ToVector(Float) (Variables|Don'ttouchme!!|GetTemp%20Size))))
        (bind _returnvalue_3 (Effects|SpawnEmitterAttached (Variables|Don'ttouchme!!|GetTemp%20Particle) _meshcomponent (Variables|GoodParticleStatusSettingInput|GetLeft%20Hand%20Point%20Name) "0, 0, 0" "0, 0, 0" (Math|Conversions|ToVector(Float) (Variables|Don'ttouchme!!|GetTemp%20Size))))
        (Variables|Don'ttouchme!!|SetNow%20Particle (Utilities|Array|MakeArray _returnvalue_3 _returnvalue_2))
        ;[1 1 1] Add Power up
        (bind _meshcomponent_2 (CallFunction|FindMesh))
        (Effects|SpawnEmitterAttached "/Game/GoodParticleStatus/Particles/Buff_Status/PS_GPS_Buff_PowerUp.PS_GPS_Buff_PowerUp" _meshcomponent_2 (Variables|GoodParticleStatusSettingInput|GetRoot%20Point%20Name) "0, 0, 0" "0, 0, 0" (Math|Conversions|ToVector(Float) (Variables|Don'ttouchme!!|GetTemp%20Size))))
      (:NewEnumerator3
        (Variables|Don'ttouchme!!|SetTemp%20Particle (Variables|GoodParticleStatusParticleSetting|GetBuff%20:%20Fire))
        (goto _label))
      (:NewEnumerator15
        (Variables|Don'ttouchme!!|SetTemp%20Particle (Variables|GoodParticleStatusParticleSetting|GetBuff%20:%20Nebula))
        (goto _label))
      (:NewEnumerator1
        (Variables|Don'ttouchme!!|SetTemp%20Particle (Variables|GoodParticleStatusParticleSetting|GetBuff%20:%20Trail%20Ice))
        (goto _label))
      (:NewEnumerator8
        (Variables|Don'ttouchme!!|SetTemp%20Particle (Variables|GoodParticleStatusParticleSetting|GetBuff%20:%20Trail%20Poison))
        (goto _label))
      (:NewEnumerator0
        (Variables|Don'ttouchme!!|SetTemp%20Particle (Variables|GoodParticleStatusParticleSetting|GetBuff%20:%20Trail%20Soft))
        (goto _label))
      (:NewEnumerator17
        (Variables|Don'ttouchme!!|SetTemp%20Particle (Variables|GoodParticleStatusParticleSetting|GetBuff%20:%20Trail%20Sparks))
        (goto _label))
      (:NewEnumerator18
        (Variables|Don'ttouchme!!|SetTemp%20Particle (Variables|GoodParticleStatusParticleSetting|GetBuff%20:%20Trail%20Spirit%20Wave))
        (goto _label))
      (:NewEnumerator25
        (Variables|Don'ttouchme!!|SetTemp%20Particle (Variables|GoodParticleStatusParticleSetting|GetBuff%20:%20DarkFlame))
        (goto _label))
      (:NewEnumerator6
        ;[1 1 1] Head
        (Variables|Don'ttouchme!!|SetTemp%20Particle (Variables|GoodParticleStatusParticleSetting|GetHead%20:%20Chaos))
        (Variables|Don'ttouchme!!|SetTemp%20Point%20Name (Variables|GoodParticleStatusSettingInput|GetAbove%20The%20Head%20Point%20Name) :!label _label_2)
        (Variables|Don'ttouchme!!|SetTemp%20Size (Variables|GoodParticleStatusSettingInput|GetParticle%20Size) :!label _label_3)
        (bind _meshcomponent_3 (CallFunction|FindMesh))
        (bind _returnvalue_4 (Effects|SpawnEmitterAttached (Variables|Don'ttouchme!!|GetTemp%20Particle) _meshcomponent_3 (Variables|Don'ttouchme!!|GetTemp%20Point%20Name) "0, 0, 0" "0, 0, 0" (Math|Conversions|ToVector(Float) (Variables|Don'ttouchme!!|GetTemp%20Size))))
        (Variables|Don'ttouchme!!|SetNow%20Particle (Utilities|Array|MakeArray _returnvalue_4)))
      (:NewEnumerator27
        (Variables|Don'ttouchme!!|SetTemp%20Particle (Variables|GoodParticleStatusParticleSetting|GetHead%20:%20Eagle%20Vision))
        (goto _label_2))
      (:NewEnumerator21
        (Variables|Don'ttouchme!!|SetTemp%20Particle (Variables|GoodParticleStatusParticleSetting|GetHead%20:%20Evil))
        (goto _label_2))
      (:NewEnumerator22
        (Variables|Don'ttouchme!!|SetTemp%20Particle (Variables|GoodParticleStatusParticleSetting|GetHead%20:%20Exclamation%20Mark))
        (goto _label_2))
      (:NewEnumerator26
        (Variables|Don'ttouchme!!|SetTemp%20Particle (Variables|GoodParticleStatusParticleSetting|GetHead%20:Heart))
        (goto _label_2))
      (:NewEnumerator23
        (Variables|Don'ttouchme!!|SetTemp%20Particle (Variables|GoodParticleStatusParticleSetting|GetHead%20:QuestionMark))
        (goto _label_2))
      (:NewEnumerator24
        (Variables|Don'ttouchme!!|SetTemp%20Particle (Variables|GoodParticleStatusParticleSetting|GetHead%20:%20Selection))
        (bind _meshcomponent_4 (CallFunction|FindMesh))
        (bind _returnvalue_5 (Effects|SpawnEmitterAttached (Variables|Don'ttouchme!!|GetTemp%20Particle) _meshcomponent_4 (Variables|GoodParticleStatusSettingInput|GetAbove%20The%20Head%20Point%20Name) "0, 0, 0" "0, 0, 0" (Math|Conversions|ToVector(Float) (Variables|Don'ttouchme!!|GetTemp%20Size))))
        (bind _returnvalue_6 (Effects|SpawnEmitterAttached "/Game/GoodParticleStatus/Particles/Head_Status/PS_GPS_Selection_02.PS_GPS_Selection_02" _meshcomponent_4 (Variables|GoodParticleStatusSettingInput|GetRoot%20Point%20Name) "0, 0, 0" "0, 0, 0" (Math|Conversions|ToVector(Float) (Variables|Don'ttouchme!!|GetTemp%20Size))))
        (Variables|Don'ttouchme!!|SetNow%20Particle (Utilities|Array|MakeArray _returnvalue_6 _returnvalue_5)))
      (:NewEnumerator7
        (Variables|Don'ttouchme!!|SetTemp%20Particle (Variables|GoodParticleStatusParticleSetting|GetHead%20:%20Slience))
        (goto _label_2))
      (:NewEnumerator5
        (Variables|Don'ttouchme!!|SetTemp%20Particle (Variables|GoodParticleStatusParticleSetting|GetHead%20:%20Sleep%20))
        (goto _label_2))
      (:NewEnumerator4
        (Variables|Don'ttouchme!!|SetTemp%20Particle (Variables|GoodParticleStatusParticleSetting|GetHead%20:%20Stun%20))
        (goto _label_2))
      (:NewEnumerator19
        (Variables|Don'ttouchme!!|SetTemp%20Particle (Variables|GoodParticleStatusParticleSetting|GetHead%20:Unlucky%20))
        (goto _label_2))
      (:NewEnumerator14
        ;[1 1 1] Status
        (Variables|Don'ttouchme!!|SetTemp%20Particle (Variables|GoodParticleStatusParticleSetting|GetStatus%20:%20Shield%20Fire))
        (Variables|Don'ttouchme!!|SetTemp%20Point%20Name (Variables|GoodParticleStatusSettingInput|GetBody%20Center%20Point%20Name) :!label _label_4)
        (goto _label_3))
      (:NewEnumerator20
        (Variables|Don'ttouchme!!|SetTemp%20Particle (Variables|GoodParticleStatusParticleSetting|GetStatus%20:%20Shield%20HiTech))
        (goto _label_4))
      (:NewEnumerator13
        (Variables|Don'ttouchme!!|SetTemp%20Particle (Variables|GoodParticleStatusParticleSetting|GetStatus%20:%20Shield%20Water))
        (goto _label_4))
      (:NewEnumerator12
        (Variables|Don'ttouchme!!|SetTemp%20Particle (Variables|GoodParticleStatusParticleSetting|GetStatus%20:%20Shield%20))
        (goto _label_4))
      (:NewEnumerator10
        (Variables|Don'ttouchme!!|SetTemp%20Particle (Variables|GoodParticleStatusParticleSetting|GetDebuff%20Status%20:%20Burning))
        (goto _label_4))
      (:NewEnumerator11
        ;[1 1 1] Root : Status
        (Variables|Don'ttouchme!!|SetTemp%20Size (Variables|GoodParticleStatusSettingInput|GetParticle%20Size))
        (bind _meshcomponent_5 (CallFunction|FindMesh))
        (bind _returnvalue_7 (Effects|SpawnEmitterAttached (Variables|GoodParticleStatusParticleSetting|GetDeBuff%20:%20Frozen%20Particle) _meshcomponent_5 (Variables|GoodParticleStatusSettingInput|GetBody%20Center%20Point%20Name) "0, 0, 0" "0, 0, 0" (Math|Conversions|ToVector(Float) (Variables|Don'ttouchme!!|GetTemp%20Size))))
        (bind _returnvalue_8 (Effects|SpawnEmitterAttached "/Game/GoodParticleStatus/Particles/Status/Debuff_Status/PS_GPS_Frozen_02.PS_GPS_Frozen_02" _meshcomponent_5 (Variables|GoodParticleStatusSettingInput|GetRoot%20Point%20Name) "0, 0, 0" "0, 0, 0" (Math|Conversions|ToVector(Float) (Variables|Don'ttouchme!!|GetTemp%20Size))))
        (Variables|Don'ttouchme!!|SetNow%20Particle (Utilities|Array|MakeArray _returnvalue_8 _returnvalue_7)))
      (:NewEnumerator32
        (Variables|Don'ttouchme!!|SetTemp%20Particle (Variables|GoodParticleStatusParticleSetting|GetStatus%20:%20Backfire))
        (goto _label_4))
      (:NewEnumerator33
        (Variables|Don'ttouchme!!|SetTemp%20Particle (Variables|GoodParticleStatusParticleSetting|GetDebuff%20Status%20:%20Tar))
        (Variables|Don'ttouchme!!|SetTemp%20Point%20Name (Variables|GoodParticleStatusSettingInput|GetRoot%20Point%20Name))
        (goto _label_3))
      (:NewEnumerator34
        (Variables|Don'ttouchme!!|SetTemp%20Particle (Variables|GoodParticleStatusParticleSetting|GetDebuff%20Status%20:%20Chill))
        (bind _meshcomponent_6 (CallFunction|FindMesh))
        (bind _returnvalue_9 (Effects|SpawnEmitterAttached (Variables|Don'ttouchme!!|GetTemp%20Particle) _meshcomponent_6 (Variables|GoodParticleStatusSettingInput|GetBody%20Center%20Point%20Name) "0, 0, 0" "0, 0, 0" _returnvalue))
        (bind _returnvalue_10 (Effects|SpawnEmitterAttached "/Game/GoodParticleStatus/Particles/Status/Debuff_Status/PS_GPS_Chill_02.PS_GPS_Chill_02" _meshcomponent_6 (Variables|GoodParticleStatusSettingInput|GetRoot%20Point%20Name) "0, 0, 0" "0, 0, 0" _returnvalue))
        (Variables|Don'ttouchme!!|SetNow%20Particle (Utilities|Array|MakeArray _returnvalue_10 _returnvalue_9)))
      (:NewEnumerator28
        (Variables|Don'ttouchme!!|SetTemp%20Particle (Variables|GoodParticleStatusParticleSetting|GetRoot%20:%20Lake))
        (Variables|Don'ttouchme!!|SetTemp%20Point%20Name (Variables|GoodParticleStatusSettingInput|GetRoot%20Point%20Name) :!label _label_5)
        (goto _label_3))
      (:NewEnumerator29
        (Variables|Don'ttouchme!!|SetTemp%20Particle (Variables|GoodParticleStatusParticleSetting|GetRoot%20:%20Lava))
        (goto _label_5))
      (:NewEnumerator30
        (Variables|Don'ttouchme!!|SetTemp%20Particle (Variables|GoodParticleStatusParticleSetting|GetRoot%20:%20Snow))
        (goto _label_5))
      (:NewEnumerator31
        (Variables|Don'ttouchme!!|SetTemp%20Particle (Variables|GoodParticleStatusParticleSetting|GetRoot%20:%20Swamp))
        (goto _label_5)))))

(fn FindMesh
  (bind _ascharacter (Utilities|Casting|CastToCharacter (Components|GetOwner)))
  (return (Variables|/Script/Engine.Character|GetMesh _ascharacter)))