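; AK-74 weapon Blueprint that fires automatically while shooting and offers an aim-down-sights alternate fire.
; A successful parent TryMakeShot starts a looping timer at the shots-per-second rate, and stopping or an empty clip clears it.
; Each shot spends ammo, runs a line trace, triggers FX and plays the shooting montage.
; Alternate fire blends the view to the weapon with a narrowed camera FOV, then back to the player.
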(event Custom|StartBurst
  (CallFunction|MakeOneShot)
  (bind _returnvalue (Utilities|Time|SetTimerbyEvent (delegate Custom|MakeOneShot) (/ 1.0 (Variables|Default|GetShotPerSecond)) true))
  (Variables|Default|SetBurs_TH _returnvalue))

(event Custom|StartAlternateFire
  (Game|Player|SetViewTargetwithBlend (Game|GetPlayerController 0) self 0.2 "VTBlend_Linear" 0.0 false)
  (Camera|SetFieldOfView (Variables|Default|GetCamera) 5e+01))

(event Custom|StopAlternateFire
  (Game|Player|SetViewTargetwithBlend (Game|GetPlayerController 0) (Game|GetPlayerCharacter 0) 0.2 "VTBlend_Linear" 0.0 false)
  (Camera|SetFieldOfView (Variables|Default|GetCamera) 9e+01))

(event Custom|StopBurst
  (Utilities|Time|ClearandInvalidateTimerbyHandle (Variables|Default|GetBurs_TH)))

(event Custom|MakeOneShot
  (if (> (.inclip (Variables|/Game/-RLS/Blueprints/Components/BP_AmmoComp.BP_AmmoComp_C|GetAmmo_AK74 (Variables|Default|GetAmmoComp))) 0)
    (CallFunction|SpendAmmo)
    (CallFunction|MakeLineTraceShot)
    (CallFunction|ActivateShotFX)
    (Animation|Montage|PlayMontage (Variables|Default|GetWeaponMesh) "/Game/FPS_Assault_Pack/Animations/RU74/A_RU74_Shoot01_Montage.A_RU74_Shoot01_Montage")
    (else
      (CallFunction|StopBurst))))

(fn ConstructionScript
  (|CallParentFunction))

(fn TryMakeShot
  (bind _result (|CallParentFunction))
  (if _result
    (CallFunction|StartBurst)
    (return true)
    (else
      (Utilities|Time|ClearandInvalidateTimerbyHandle (Variables|Default|GetBurs_TH))
      (return false))))

(fn StopShooting
  (CallFunction|StopBurst)
  (|CallParentFunction))