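; Pistol weapon Blueprint that adds single-shot firing behavior on top of a parent weapon class.
; Its TryMakeShot override calls Shot only when the parent check passes, then reports whether the shot happened.
; Shot spends ammo, makes a line trace shot, activates effects and plays the pistol shot montage on the weapon mesh at half speed.
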(event Custom|Shot
  (CallFunction|SpendAmmo)
  (CallFunction|MakeLineTraceShot)
  (CallFunction|ActivateFX)
  (Animation|Montage|PlayMontage (Variables|Default|GetWeaponMesh) "/Game/pistol1911/Weapon/Animations/anim_pistol191_shot.anim_pistol191_shot" 0.5))

(fn ConstructionScript
  (|CallParentFunction))

(fn TryMakeShot
  (bind _result (|CallParentFunction))
  (if _result
    (CallFunction|Shot)
    (return true)
    (else
      (return false))))