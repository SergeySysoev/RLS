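; Base weapon Blueprint providing hitscan firing, shot FX, a reload montage and ammo hooks for six gun types.
; MakeLineTraceShot traces from the player camera within a random scatter cone, fires OnShot, then spawns BP_ImpactEffect and applies point damage on a blocking hit.
; An injected ammo component holds per-type clip counts, selected by the weapon's enum for shot checks and spending.
; StopShooting is effectively a stub, and the debug line drawing never runs.
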(event Custom|ApplyReloadMontage
  (Animation|Montage|PlayMontage (Variables|Default|GetWeaponMesh) (Variables|-EditableVariables|GetWeapon_ReloadMontage)))

(event EventBeginPlay
  (Variables|-Runtimevariable|SetCurrentAmmo (Variables|-EditableVariables|GetTotalAmmo)))

(fn ConstructionScript)

(fn TryMakeShot
  (bind _ammocomp (Variables|Default|GetAmmoComp))
  (return (> (Utilities|Select :Index (Variables|-EditableVariables|GetNameEnum) :NewEnumerator0 (.inclip (Variables|/Game/-RLS/Blueprints/Components/BP_AmmoComp.BP_AmmoComp_C|GetAmmo_M16 _ammocomp)) :NewEnumerator1 (.inclip (Variables|/Game/-RLS/Blueprints/Components/BP_AmmoComp.BP_AmmoComp_C|GetAmmo_AK74 _ammocomp)) :NewEnumerator2 (.inclip (Variables|/Game/-RLS/Blueprints/Components/BP_AmmoComp.BP_AmmoComp_C|GetAmmo_Shotgun _ammocomp)) :NewEnumerator3 (.inclip (Variables|/Game/-RLS/Blueprints/Components/BP_AmmoComp.BP_AmmoComp_C|GetAmmo_RL _ammocomp)) :NewEnumerator4 (.inclip (Variables|/Game/-RLS/Blueprints/Components/BP_AmmoComp.BP_AmmoComp_C|GetAmmo_Pistol _ammocomp)) :NewEnumerator5 (.inclip (Variables|/Game/-RLS/Blueprints/Components/BP_AmmoComp.BP_AmmoComp_C|GetAmmo_DBShotgun _ammocomp))) 0)))

(fn StopShooting
  (if (== (Variables|-Runtimevariable|GetCurrentAmmo) 0)
    (return)))

(fn MakeLineTraceShot
  (bind _returnvalue (Game|GetPlayerCameraManager 0))
  (bind _returnvalue_2 (Camera|GetCameraLocation _returnvalue))
  (bind _outhit (Collision|LineTraceByChannel _returnvalue_2 (+ _returnvalue_2 (* (Math|Random|RandomUnitVectorinConeinDegrees (Transformation|GetActorForwardVector _returnvalue) (Variables|-EditableVariables|GetScatter)) (Variables|-EditableVariables|GetShotDistance))) "TraceTypeQuery1" true 0 "None"))
  (Default|CallOnShot)
  (if (.bBlockingHit (Collision|BreakHitResult _outhit))
    (bind _returnvalue_3 (Game|SpawnActorfromClass "/Game/-RLS/Blueprints/Damage/BP_ImpactEffect.BP_ImpactEffect_C" (Math|Transform|MakeTransform (.ImpactPoint (Collision|BreakHitResult _outhit)) "0, 0, 0" "1,1,1") "Undefined" 0 0))
    (Default|InitIE _returnvalue_3 _outhit)
    (Game|Damage|ApplyPointDamage (.HitActor (Collision|BreakHitResult _outhit)) (Variables|-EditableVariables|GetDamage) (Math|Vector|Normalize (- (.TraceEnd (Collision|BreakHitResult _outhit)) (.TraceStart (Collision|BreakHitResult _outhit)))) _outhit (Game|GetPlayerController 0) self (Variables|-EditableVariables|GetDamageType))))

(fn ActivateShotFX
  (Components|Activation|Activate (Variables|Default|GetShotSound) true))

(fn SetAmmoComp
  (params (AmmoComp :type BP%20Ammo%20Comp%20Object%20Reference))
  (bind _output_get (Variables|Default|SetAmmoComp AmmoComp))
  (Variables|-Runtimevariable|SetCurrentAmmo (Utilities|Select :Index (Variables|-EditableVariables|GetNameEnum) :NewEnumerator0 (.inclip (Variables|/Game/-RLS/Blueprints/Components/BP_AmmoComp.BP_AmmoComp_C|GetAmmo_M16 _output_get)) :NewEnumerator1 (.inclip (Variables|/Game/-RLS/Blueprints/Components/BP_AmmoComp.BP_AmmoComp_C|GetAmmo_AK74 _output_get)) :NewEnumerator2 (.inclip (Variables|/Game/-RLS/Blueprints/Components/BP_AmmoComp.BP_AmmoComp_C|GetAmmo_Shotgun _output_get)) :NewEnumerator3 (.inclip (Variables|/Game/-RLS/Blueprints/Components/BP_AmmoComp.BP_AmmoComp_C|GetAmmo_RL _output_get)) :NewEnumerator4 (.inclip (Variables|/Game/-RLS/Blueprints/Components/BP_AmmoComp.BP_AmmoComp_C|GetAmmo_Pistol _output_get)) :NewEnumerator5 (.inclip (Variables|/Game/-RLS/Blueprints/Components/BP_AmmoComp.BP_AmmoComp_C|GetAmmo_DBShotgun _output_get)))))

(fn SpendAmmo
  (Default|SpendAmmo (Variables|Default|GetAmmoComp) (Variables|-EditableVariables|GetNameEnum)))