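; M16 rifle weapon Blueprint that adds hitscan firing and scoped aiming on top of a parent weapon class.
; When the parent's TryMakeShot check passes, MakeShot spends ammo, runs a line trace, triggers shot FX and plays a shooting montage on the weapon mesh.
; Alternate fire blends the first player's view to the weapon and narrows ScopeCamera's field of view, then restores both on stop.
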(event Custom|MakeShot
  (CallFunction|SpendAmmo)
  (CallFunction|MakeLineTraceShot)
  (CallFunction|ActivateShotFX)
  (Animation|Montage|PlayMontage (Variables|Default|GetWeaponMesh) "/Game/FPS_Assault_Pack/Animations/Rifle/A_Rifle_Shoot01_Montage.A_Rifle_Shoot01_Montage"))

(event Custom|StartAlternateFire
  (Game|Player|SetViewTargetwithBlend (Game|GetPlayerController 0) self 0.2 "VTBlend_Linear" 0.0 false)
  (Camera|SetFieldOfView (Variables|Default|GetScopeCamera) 5e+01))

(event Custom|StopAlternateFire
  (Game|Player|SetViewTargetwithBlend (Game|GetPlayerController 0) (Game|GetPlayerCharacter 0) 0.2 "VTBlend_Linear" 0.0 false)
  (Camera|SetFieldOfView (Variables|Default|GetScopeCamera) 9e+01))

(fn ConstructionScript
  (|CallParentFunction))

(fn TryMakeShot
  (bind _result (|CallParentFunction))
  (if _result
    (CallFunction|MakeShot)
    (return true)
    (else
      (return false))))