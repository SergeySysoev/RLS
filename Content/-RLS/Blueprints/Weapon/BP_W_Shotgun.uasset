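; Shotgun weapon Blueprint that fires each shot as a timed burst of pellet subshots from a single ammo spend.
; TryMakeShot extends the parent check and starts the shot, which plays FX and a fire montage.
; A looping timer drives the subshots, each firing several line traces with scatter widened in proportion to its index.
; CanShoot blocks refiring until the montage completes or a fallback delay elapses.
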(event Custom|MakeSubshot
  (Math|Integer|IncrementInt (Variables|Default|GetCurrentSubshot)
    (:%20%20
      (if (>= (Variables|Default|GetSubshotCount) (Variables|Default|GetCurrentSubshot))
        (Variables|Default|SetScatter (* (Variables|Default|GetCurrentSubshot) (Variables|Default|GetDefaultScatter)))
        (for _index (range 1 (Variables|Default|GetPelletInSubshot))
          (CallFunction|MakeLineTraceShot))
        (else
          (Utilities|Time|ClearandInvalidateTimerbyHandle (Variables|Default|GetSubshot_TH))
          (Variables|Default|SetCurrentSubshot 0))))))

(event Custom|StartShot
  (if (Variables|Default|GetCanShoot)
    (Utilities|FlowControl|Sequence
      (:then_0
        (Variables|Default|SetCanShoot false)
        (CallFunction|SpendAmmo)
        (CallFunction|MakeSubshot)
        (bind _returnvalue (Utilities|Time|SetTimerbyEvent (delegate Custom|MakeSubshot) (Variables|Default|GetSubshotDelay) true))
        (Variables|Default|SetSubshot_TH _returnvalue)
        (CallFunction|ActivateShotFX)
        (Animation|Montage|PlayMontage (Variables|Default|GetWeaponMesh) "/Game/MilitaryWeapDark/Weapons/Anims/Fire_Shotgun_Silent_Montage1.Fire_Shotgun_Silent_Montage1"
          (:OnCompleted
            (Variables|Default|SetCanShoot true))))
      (:then_1
        (Utilities|FlowControl|Delay 1.5)
        (Variables|Default|SetCanShoot true)))))

(event EventBeginPlay
  (|CallParentFunction)
  (Variables|Default|SetDefaultScatter (Variables|Default|GetScatter)))

(fn ConstructionScript
  (|CallParentFunction))

(fn TryMakeShot
  (bind _result (|CallParentFunction))
  (if _result
    (CallFunction|StartShot)
    (return true)
    (else
      (return false))))