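; Double-barrel shotgun weapon that extends a parent weapon's shot and reload behavior.
; A successful TryMakeShot calls StartShot, which spends ammo, plays FX and montage, and gates firing until montage completion or a fallback delay.
; A looping timer staggers each shot into subshots of multiple line-trace pellets, scaling scatter up from its default with each subshot.
; Reload montage depends on shells left in the clip.
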(event Custom|MakeSubshot
  (Math|Integer|IncrementInt (Variables|Default|GetCurrentSubshot)
    (:%20%20
      (if (>= (Variables|Default|GetSubshotCount) (Variables|Default|GetCurrentSubshot))
        (Variables|Default|SetScatter (* (Variables|Default|GetCurrentSubshot) (Variables|Default|GetDefaultScatter)))
        (for _index (range 1 (Variables|Default|GetPelletInSubshot))
          (CallFunction|MakeLineTraceShot))
        (else
          (Utilities|Time|ClearandInvalidateTimerbyHandle (Variables|Default|GetSubshot_TH))
          (Variables|Default|SetCurrentSubshot 0))))))

(event Custom|StartShot
  (if (Variables|Default|GetCanShoot)
    (Utilities|FlowControl|Sequence
      (:then_0
        (Variables|Default|SetCanShoot false)
        (CallFunction|SpendAmmo)
        (CallFunction|MakeSubshot)
        (bind _returnvalue (Utilities|Time|SetTimerbyEvent (delegate Custom|MakeSubshot) (Variables|Default|GetSubshotDelay) true))
        (Variables|Default|SetSubshot_TH _returnvalue)
        (CallFunction|ActivateShotFX)
        (Animation|Montage|PlayMontage (Variables|Default|GetWeaponMesh) "/Game/Animated_DBShotgun/anims/dbshotgun/ANIM_dbshotgun_shoot_01_Montage.ANIM_dbshotgun_shoot_01_Montage"
          (:OnCompleted
            (Variables|Default|SetCanShoot true))))
      (:then_1
        (Utilities|FlowControl|Delay 1.5)
        (Variables|Default|SetCanShoot true)))))

(event Custom|MakeShot
  (CallFunction|SpendAmmo)
  (CallFunction|MakeLineTraceShot)
  (CallFunction|ActivateShotFX)
  (Animation|Montage|PlayMontage (Variables|Default|GetWeaponMesh) "/Game/Animated_DBShotgun/anims/dbshotgun/ANIM_dbshotgun_shoot_01_Montage.ANIM_dbshotgun_shoot_01_Montage"))

(event EventBeginPlay
  (|CallParentFunction)
  (Variables|Default|SetDefaultScatter (Variables|Default|GetScatter)))

(event EventApplyReloadMontage
  (switch int (.InClip (Utilities|Struct|BreakStruct_WeaponAmmo (Variables|/Game/-RLS/Blueprints/Components/BP_AmmoComp.BP_AmmoComp_C|GetAmmo_DBShotgun (Variables|Default|GetAmmoComp))))
    (:0
      (Animation|Montage|PlayMontage (Variables|Default|GetWeaponMesh) "/Game/Animated_DBShotgun/anims/dbshotgun/ANIM_dbshotgun_reload_02_Montage.ANIM_dbshotgun_reload_02_Montage"))
    (:1
      (Animation|Montage|PlayMontage (Variables|Default|GetWeaponMesh) (Variables|Default|GetWeapon_ReloadMontage)))))

(fn ConstructionScript
  (|CallParentFunction))

(fn TryMakeShot
  (bind _result (|CallParentFunction))
  (if _result
    (CallFunction|StartShot)
    (return true)
    (else
      (return false))))