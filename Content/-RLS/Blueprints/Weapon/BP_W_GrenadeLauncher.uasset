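; Grenade launcher weapon Blueprint that fires a projectile along the player camera's aim when a shot is allowed.
; TryMakeShot defers to the parent weapon check, then calls Shot, which spawns the projectile class at the WeaponDir component using the camera rotation.
; Each shot triggers FX, the OnShot call and ammo spend, then a WeaponReady flag and Delay enforce a one-second cooldown.
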(event Custom|Shot
  (if (Variables|Default|GetWeaponReady)
    (Game|SpawnActorfromClass (Variables|Default|GetProjectileClass) (Math|Transform|MakeTransform (.location (Transformation|GetWorldTransform (Variables|Default|GetWeaponDir))) (Camera|GetCameraRotation (Game|GetPlayerCameraManager 0)) "1,1,1") "AlwaysSpawn" 0 0)
    (CallFunction|ActivateShotFX)
    (Default|CallOnShot)
    (CallFunction|SpendAmmo)
    (Variables|Default|SetWeaponReady false)
    (Utilities|FlowControl|Delay 1.0)
    (Variables|Default|SetWeaponReady true)))

(event EventBeginPlay
  (|CallParentFunction) ; This node is disabled and will not be called.\nDrag off pins to build functionality.
)

(event Collision|EventActorBeginOverlap
  (params (OtherActor :type Actor%20Object%20Reference))
  (|CallParentFunction OtherActor) ; This node is disabled and will not be called.\nDrag off pins to build functionality.
)

(event EventTick
  (params (DeltaSeconds :type Float%20%28single-precision%29))
  (|CallParentFunction DeltaSeconds) ; This node is disabled and will not be called.\nDrag off pins to build functionality.
)

(fn ConstructionScript
  (|CallParentFunction))

(fn TryMakeShot
  (bind _result (|CallParentFunction))
  (if _result
    (CallFunction|Shot)
    (return true)
    (else
      (return false))))