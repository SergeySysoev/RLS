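; Rocket projectile Blueprint that explodes on impact, with small frag explosion particles and sound at its location.
; Both a collision component hit and the Destroyed event call Explode, which spawns the effects and then destroys the actor.
; A DoOnce gate keeps the resulting Destroyed callback from repeating the explosion, so it also explodes once when destroyed by other means.
; This graph applies no damage itself.
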(event OnComponentHit(ProjectileCollision)
  (params (HitComponent :type Primitive%20Component%20Object%20Reference) (OtherActor :type Actor%20Object%20Reference) (OtherComp :type Primitive%20Component%20Object%20Reference) (NormalImpulse :type Vector :default "0, 0, 0") (Hit :type Hit%20Result%20Structure%20%28by%20ref%29))
  (CallFunction|Explode))

(event Custom|Explode
  (bind _returnvalue (Transformation|GetActorLocation))
  (Utilities|FlowControl|DoOnce false
    (:Completed
      (Utilities|FlowControl|Sequence
        (:then_0
          (Effects|SpawnEmitteratLocation "/Game/BallisticsVFX/Particles/Explosive/Explosion_Frag_small.Explosion_Frag_small" _returnvalue)
          (Audio|SpawnSoundatLocation "/Game/BallisticsVFX/SFX/Explodes/Explosions_frag.Explosions_frag" _returnvalue "0, 0, 0" 1.0 1.0 0.0 0 0))
        (:then_1
          (Actor|DestroyActor))))))

(event EventBeginPlay
  (|CallParentFunction))

(event Collision|EventActorBeginOverlap
  (params (OtherActor :type Actor%20Object%20Reference))
  (|CallParentFunction OtherActor) ; This node is disabled and will not be called.\nDrag off pins to build functionality.
)

(event EventTick
  (params (DeltaSeconds :type Float%20%28single-precision%29))
  (|CallParentFunction DeltaSeconds) ; This node is disabled and will not be called.\nDrag off pins to build functionality.
)

(event EventDestroyed
  (CallFunction|Explode))

(fn ConstructionScript
  (|CallParentFunction))