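; BP_FigureDrawer is an actor that draws a debug square, cube and five-pointed star in a row from its location on BeginPlay.
; DrawSquare chains lines along the actor's forward and right vectors and returns its corner points.
; DrawCube reuses DrawSquare for bottom and top faces, then joins matching corners with vertical edges.
; DrawStar repeatedly draws a segment and rotates its direction 144 degrees around world Z.
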(event EventBeginPlay
  (bind _returnvalue (Transformation|GetActorLocation))
  (bind _returnvalue_2 (+ _returnvalue "200.000000, 0, 0"))
  (CallFunction|DrawSquare _returnvalue 1e+02)
  (CallFunction|DrawCube _returnvalue_2 1e+02)
  (CallFunction|DrawStar (+ _returnvalue_2 "200.000000, 0, 0") 1e+02))

(fn ConstructionScript)

(fn DrawSquare
  (params (StartPoint :type Vector) (SideLength :type Float%20%28single-precision%29))
  (bind _returnvalue (Transformation|GetActorRightVector))
  (Utilities|FlowControl|Sequence
    (:then_0
      (bind _output_get (LocalVariables|SetLocal_NextStartPoint StartPoint))
      (bind _output_get_2 (LocalVariables|SetLocal_SideLength SideLength))
      (bind _output_get_3 (LocalVariables|SetLocal_NextEndPoint (+ _output_get (* (Transformation|GetActorForwardVector) _output_get_2))))
      (Utilities|Array|Add (LocalVariables|GetLocal_SquarePoints) _output_get_3))
    (:then_1
      (for _index (range 0 3)
        (Rendering|Debug|DrawDebugLine (LocalVariables|GetLocal_NextStartPoint) (LocalVariables|GetLocal_NextEndPoint) (Variables|Default|GetDrawColor) (Variables|Default|GetDrawDuration) (Variables|Default|GetLineThickness))
        (if (< _index 3)
          (bind _output_get_4 (LocalVariables|SetLocal_NextStartPoint (LocalVariables|GetLocal_NextEndPoint)))
          (bind _output_get_5 (LocalVariables|SetLocal_NextEndPoint (+ _output_get_4 (* (Utilities|Select :Index _index :Option%200 _returnvalue :Option%201 (* (Transformation|GetActorForwardVector) -1.0) :Option%202 (* _returnvalue -1.0)) (LocalVariables|GetLocal_SideLength)))))
          (Utilities|Array|Add (LocalVariables|GetLocal_SquarePoints) _output_get_5))))
    (:then_2
      (return (LocalVariables|GetLocal_SquarePoints)))))

(fn DrawCube
  (params (StartPoint :type Vector) (SideLength :type Float%20%28single-precision%29))
  (Utilities|FlowControl|Sequence
    (:then_0
      (bind _squarepoints (CallFunction|DrawSquare StartPoint SideLength))
      (LocalVariables|SetLocal_StartPoints _squarepoints))
    (:then_1
      (bind _squarepoints_2 (CallFunction|DrawSquare (+ StartPoint (* (Transformation|GetActorUpVector) SideLength)) SideLength))
      (LocalVariables|SetLocal_EndPoints _squarepoints_2))
    (:then_2
      (for (_array_element _array_index) (LocalVariables|GetLocal_StartPoints)
        (Rendering|Debug|DrawDebugLine _array_element (Utilities|Array|Get(acopy) (LocalVariables|GetLocal_EndPoints) _array_index) (Variables|Default|GetDrawColor) (Variables|Default|GetDrawDuration) (Variables|Default|GetLineThickness))))))

(fn DrawStar
  (params (StartPoint :type Vector) (SideLength :type Float%20%28single-precision%29))
  (Utilities|FlowControl|Sequence
    (:then_0
      (LocalVariables|SetLocal_StartPoint StartPoint)
      (LocalVariables|SetLocal_SideLength SideLength)
      (LocalVariables|SetLocal_Direction (Transformation|GetActorForwardVector)))
    (:then_1
      (for _index (range 0 4)
        (Rendering|Debug|DrawDebugLine (LocalVariables|GetLocal_StartPoint) (+ (LocalVariables|GetLocal_StartPoint) (* (LocalVariables|GetLocal_Direction) (LocalVariables|GetLocal_SideLength))) (Variables|Default|GetDrawColor) (Variables|Default|GetDrawDuration) (Variables|Default|GetLineThickness))
        (LocalVariables|SetLocal_StartPoint (+ (LocalVariables|GetLocal_StartPoint) (* (LocalVariables|GetLocal_Direction) (LocalVariables|GetLocal_SideLength))))
        (LocalVariables|SetLocal_Direction (Math|Vector|RotateVectorAroundAxis (LocalVariables|GetLocal_Direction) 144.0 "0, 0,1.000000"))))))