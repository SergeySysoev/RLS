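; BP_ColorBox is an environment actor that changes the opacity of its Sphere component according to how far away a target is.
; Each Tick it reads DistanceToTarget from its BPTargetCheckComponent, clamps it between MinDistance and MaxDistance, and normalizes it to a zero-to-one value.
; That value drives the Opacity scalar parameter on the Sphere's materials, so opacity rises as the distance grows.
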(event EventBeginPlay)

(event Collision|EventActorBeginOverlap
  (params (OtherActor :type Actor%20Object%20Reference)))

(event EventTick
  (params (DeltaSeconds :type Float%20%28single-precision%29))
  (Rendering|Material|SetScalarParameterValueonMaterials (Variables|Default|GetSphere) "Opacity" (/ (- (Math|Float|Clamp(Float) (Variables|/Game/-RLS/Blueprints/Components/BP_TargetCheck_Component.BP_TargetCheck_Component_C|GetDistanceToTarget (Variables|Default|GetBP_TargetCheck_Component)) (Variables|-Edittablevariables|GetMinDistance) (Variables|-Edittablevariables|GetMaxDistance)) (Variables|-Edittablevariables|GetMinDistance)) (- (Variables|-Edittablevariables|GetMaxDistance) (Variables|-Edittablevariables|GetMinDistance)))))

(fn ConstructionScript)