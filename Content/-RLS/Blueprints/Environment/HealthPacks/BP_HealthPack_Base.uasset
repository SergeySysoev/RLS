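; Base health pack pickup that spins in place and heals the player character on overlap.
; Overlap matches the player by display name and proceeds only if current HP is below a hard-coded 100.
; It plays the pickup sound, waits out its duration, then Heal restores a share of total HP based on pack Size.
; CalculateHP caps the result at total HP, and the pack destroys itself after updating the vitality component.
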(event OnComponentBeginOverlap(Collision)
  (params (OverlappedComponent :type Primitive%20Component%20Object%20Reference) (OtherActor :type Actor%20Object%20Reference) (OtherComp :type Primitive%20Component%20Object%20Reference) (OtherBodyIndex :type Integer) (bFromSweep :type Boolean) (SweepResult :type Hit%20Result%20Structure%20%28by%20ref%29))
  (bind _returnvalue (Game|GetPlayerCharacter 0))
  (bind _pickupsound (Variables|Default|GetPickUpSound))
  (if (Utilities|Enum|Equal(Enum) (Utilities|GetDisplayName OtherActor) (Utilities|GetDisplayName _returnvalue))
    (bind _asbp_character (Utilities|Casting|CastToBP_Character _returnvalue))
    (if (< (Variables|/Game/-RLS/Blueprints/Components/BP_VitalityComponent.BP_VitalityComponent_C|GetCurrentHP (Variables|/Game/-RLS/Blueprints/Character/BP_Character.BP_Character_C|GetBP_VitalityComponent _asbp_character)) 1e+02)
      (Components|Activation|Activate _pickupsound true)
      (Utilities|FlowControl|Delay (Variables|/Script/Engine.SoundBase|GetDuration (Variables|/Script/Engine.AudioComponent|GetSound _pickupsound)))
      (CallFunction|Heal (Variables|/Game/-RLS/Blueprints/Character/BP_Character.BP_Character_C|GetBP_VitalityComponent _asbp_character)))))

(event EventBeginPlay)

(event Collision|EventActorBeginOverlap
  (params (OtherActor :type Actor%20Object%20Reference)))

(event EventTick
  (params (DeltaSeconds :type Float%20%28single-precision%29))
  (Transformation|AddRelativeRotation (Variables|Default|GetStaticMesh) (Math|Rotator|MakeRotator 0.0 0.0 (* DeltaSeconds 1.8e+02)) false false))

(fn ConstructionScript)

(fn Heal
  (params (VitalityComponent :type BP%20Vitality%20Component%20Object%20Reference))
  (bind _totalhp (Variables|/Game/-RLS/Blueprints/Components/BP_VitalityComponent.BP_VitalityComponent_C|GetTotalHP VitalityComponent))
  (switch Utilities|FlowControl|Switch|SwitchonEnum_HealthPack (Variables|Default|GetSize)
    (:NewEnumerator0
      (bind _current_hp (CallFunction|CalculateHP VitalityComponent 0.1))
      (Default|UpdateHP VitalityComponent _current_hp _totalhp))
    (:NewEnumerator1
      (bind _current_hp_2 (CallFunction|CalculateHP VitalityComponent 0.3))
      (Default|UpdateHP VitalityComponent _current_hp_2 _totalhp))
    (:NewEnumerator2
      (bind _current_hp_3 (CallFunction|CalculateHP VitalityComponent 0.5))
      (Default|UpdateHP VitalityComponent _current_hp_3 _totalhp)))
  (Actor|DestroyActor)
  (return))

(fn CalculateHP
  (params (Vitality :type BP%20Vitality%20Component%20Object%20Reference) (Healing%20Percent :type Float%20%28single-precision%29))
  (bind _totalhp (Variables|/Game/-RLS/Blueprints/Components/BP_VitalityComponent.BP_VitalityComponent_C|GetTotalHP Vitality))
  (if (> (+ (Variables|/Game/-RLS/Blueprints/Components/BP_VitalityComponent.BP_VitalityComponent_C|GetCurrentHP Vitality) (* _totalhp Healing%20Percent)) _totalhp)
    (bind _output_get (Variables|/Game/-RLS/Blueprints/Components/BP_VitalityComponent.BP_VitalityComponent_C|SetCurrentHP Vitality _totalhp))
    (return _output_get)
    (else
      (bind _output_get_2 (Variables|/Game/-RLS/Blueprints/Components/BP_VitalityComponent.BP_VitalityComponent_C|SetCurrentHP Vitality (+ (Variables|/Game/-RLS/Blueprints/Components/BP_VitalityComponent.BP_VitalityComponent_C|GetCurrentHP Vitality) (* _totalhp Healing%20Percent))))
      (return _output_get_2))))