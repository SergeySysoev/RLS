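; Spinning ammo backpack pickup that refills all five of the player's weapon ammo types, with amounts scaled by game difficulty.
; Box overlap identifies the player by display name, plays a sound and waits for its duration before granting ammo.
; Amounts are added to the current weapon's AmmoComp structs, using InClip rather than Total for the launcher.
; It then fires OnAmmoChange for the held weapon's type and destroys itself.
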(event OnComponentBeginOverlap(Box)
  (params (OverlappedComponent :type Primitive%20Component%20Object%20Reference) (OtherActor :type Actor%20Object%20Reference) (OtherComp :type Primitive%20Component%20Object%20Reference) (OtherBodyIndex :type Integer) (bFromSweep :type Boolean) (SweepResult :type Hit%20Result%20Structure%20%28by%20ref%29))
  (bind _returnvalue (Game|GetPlayerCharacter 0))
  (bind _audio (Variables|Default|GetAudio))
  (if (Utilities|Enum|Equal(Enum) (Utilities|GetDisplayName OtherActor) (Utilities|GetDisplayName _returnvalue))
    (bind _asbp_character (Utilities|Casting|CastToBP_Character _returnvalue))
    (bind _asbp_weapon_base (Utilities|Casting|CastToBP_Weapon_Base (Variables|/Game/-RLS/Blueprints/Character/BP_Character.BP_Character_C|GetCurrentWeapon _asbp_character)))
    (Components|Activation|Activate _audio true)
    (Utilities|FlowControl|Delay (Variables|/Script/Engine.SoundBase|GetDuration (Variables|/Script/Engine.AudioComponent|GetSound _audio)))
    (bind _asbp_gi (Utilities|Casting|CastToBP_GI (Game|GetGameInstance)))
    (switch string (Variables|/Game/-RLS/Blueprints/Core/BP_GI.BP_GI_C|GetDifficulty _asbp_gi)
      (:Easy
        (Variables|Default|SetM16_Ammo 24)
        (Variables|Default|SetAK74_Ammo 60)
        (Variables|Default|SetShotgun_Ammo 16)
        (Variables|Default|SetRL_Ammo 3)
        (Variables|Default|SetDBShotgun_Ammo 16))
      (:Medium
        (Variables|Default|SetM16_Ammo 16)
        (Variables|Default|SetAK74_Ammo 30)
        (Variables|Default|SetShotgun_Ammo 8)
        (Variables|Default|SetRL_Ammo 2)
        (Variables|Default|SetDBShotgun_Ammo 8))
      (:Hard
        (Variables|Default|SetM16_Ammo 8)
        (Variables|Default|SetAK74_Ammo 15)
        (Variables|Default|SetShotgun_Ammo 4)
        (Variables|Default|SetRL_Ammo 1)
        (Variables|Default|SetDBShotgun_Ammo 4)))
    (bind _structout (Utilities|Struct|SetmembersinStruct_WeaponAmmo (Variables|/Game/-RLS/Blueprints/Components/BP_AmmoComp.BP_AmmoComp_C|GetAmmo_M16 (Variables|/Game/-RLS/Blueprints/Weapon/BP_Weapon_Base.BP_Weapon_Base_C|GetAmmoComp _asbp_weapon_base)) (+ (Variables|Default|GetM16_Ammo) (.Total (Utilities|Struct|BreakStruct_WeaponAmmo (Variables|/Game/-RLS/Blueprints/Components/BP_AmmoComp.BP_AmmoComp_C|GetAmmo_M16 (Variables|/Game/-RLS/Blueprints/Weapon/BP_Weapon_Base.BP_Weapon_Base_C|GetAmmoComp _asbp_weapon_base)))))))
    (bind _structout_2 (Utilities|Struct|SetmembersinStruct_WeaponAmmo (Variables|/Game/-RLS/Blueprints/Components/BP_AmmoComp.BP_AmmoComp_C|GetAmmo_AK74 (Variables|/Game/-RLS/Blueprints/Weapon/BP_Weapon_Base.BP_Weapon_Base_C|GetAmmoComp _asbp_weapon_base)) (+ (Variables|Default|GetAK74_Ammo) (.Total (Utilities|Struct|BreakStruct_WeaponAmmo (Variables|/Game/-RLS/Blueprints/Components/BP_AmmoComp.BP_AmmoComp_C|GetAmmo_AK74 (Variables|/Game/-RLS/Blueprints/Weapon/BP_Weapon_Base.BP_Weapon_Base_C|GetAmmoComp _asbp_weapon_base)))))))
    (bind _structout_3 (Utilities|Struct|SetmembersinStruct_WeaponAmmo (Variables|/Game/-RLS/Blueprints/Components/BP_AmmoComp.BP_AmmoComp_C|GetAmmo_Shotgun (Variables|/Game/-RLS/Blueprints/Weapon/BP_Weapon_Base.BP_Weapon_Base_C|GetAmmoComp _asbp_weapon_base)) (+ (Variables|Default|GetShotgun_Ammo) (.Total (Utilities|Struct|BreakStruct_WeaponAmmo (Variables|/Game/-RLS/Blueprints/Components/BP_AmmoComp.BP_AmmoComp_C|GetAmmo_Shotgun (Variables|/Game/-RLS/Blueprints/Weapon/BP_Weapon_Base.BP_Weapon_Base_C|GetAmmoComp _asbp_weapon_base)))))))
    (bind _structout_4 (Utilities|Struct|SetmembersinStruct_WeaponAmmo (Variables|/Game/-RLS/Blueprints/Components/BP_AmmoComp.BP_AmmoComp_C|GetAmmo_RL (Variables|/Game/-RLS/Blueprints/Weapon/BP_Weapon_Base.BP_Weapon_Base_C|GetAmmoComp _asbp_weapon_base)) (+ (Variables|Default|GetRL_Ammo) (.InClip (Utilities|Struct|BreakStruct_WeaponAmmo (Variables|/Game/-RLS/Blueprints/Components/BP_AmmoComp.BP_AmmoComp_C|GetAmmo_RL (Variables|/Game/-RLS/Blueprints/Weapon/BP_Weapon_Base.BP_Weapon_Base_C|GetAmmoComp _asbp_weapon_base)))))))
    (bind _structout_5 (Utilities|Struct|SetmembersinStruct_WeaponAmmo (Variables|/Game/-RLS/Blueprints/Components/BP_AmmoComp.BP_AmmoComp_C|GetAmmo_DBShotgun (Variables|/Game/-RLS/Blueprints/Weapon/BP_Weapon_Base.BP_Weapon_Base_C|GetAmmoComp _asbp_weapon_base)) (+ (Variables|Default|GetDBShotgun_Ammo) (.Total (Utilities|Struct|BreakStruct_WeaponAmmo (Variables|/Game/-RLS/Blueprints/Components/BP_AmmoComp.BP_AmmoComp_C|GetAmmo_DBShotgun (Variables|/Game/-RLS/Blueprints/Weapon/BP_Weapon_Base.BP_Weapon_Base_C|GetAmmoComp _asbp_weapon_base)))))))
    (switch string (Variables|/Game/-RLS/Blueprints/Weapon/BP_Weapon_Base.BP_Weapon_Base_C|GetName (Variables|/Game/-RLS/Blueprints/Character/BP_Character.BP_Character_C|GetCurrentWeapon _asbp_character))
      (:M16
        (Default|CallOnAmmoChange (Variables|/Game/-RLS/Blueprints/Weapon/BP_Weapon_Base.BP_Weapon_Base_C|GetAmmoComp _asbp_weapon_base) _structout))
      (:AK74
        (Default|CallOnAmmoChange (Variables|/Game/-RLS/Blueprints/Weapon/BP_Weapon_Base.BP_Weapon_Base_C|GetAmmoComp _asbp_weapon_base) _structout_2))
      (:Shotgun
        (Default|CallOnAmmoChange (Variables|/Game/-RLS/Blueprints/Weapon/BP_Weapon_Base.BP_Weapon_Base_C|GetAmmoComp _asbp_weapon_base) _structout_3))
      (:GrenadeLauncher
        (Default|CallOnAmmoChange (Variables|/Game/-RLS/Blueprints/Weapon/BP_Weapon_Base.BP_Weapon_Base_C|GetAmmoComp _asbp_weapon_base) _structout_4))
      (:DBShotgun
        (Default|CallOnAmmoChange (Variables|/Game/-RLS/Blueprints/Weapon/BP_Weapon_Base.BP_Weapon_Base_C|GetAmmoComp _asbp_weapon_base) _structout_5)))
    (Actor|DestroyActor)))

(event EventBeginPlay)

(event Collision|EventActorBeginOverlap
  (params (OtherActor :type Actor%20Object%20Reference)))

(event EventTick
  (params (DeltaSeconds :type Float%20%28single-precision%29))
  (Transformation|AddRelativeRotation (Variables|Default|GetAmmo_Backpack) (Math|Rotator|MakeRotator 0.0 0.0 (* DeltaSeconds 1.8e+02)) false false))

(fn ConstructionScript)