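; AK74 ammunition actor that sets how much ammo it holds according to the game's difficulty.
; On BeginPlay it runs the parent logic, then reads Difficulty from BP_GI and sets AmmoCount, with smaller amounts on harder settings.
; The overlap and tick events are disabled stubs and the construction script only calls the parent, so any other behavior comes from the parent class.
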(event EventBeginPlay
  (|CallParentFunction)
  (bind _asbp_gi (Utilities|Casting|CastToBP_GI (Game|GetGameInstance)))
  (switch string (Variables|/Game/-RLS/Blueprints/Core/BP_GI.BP_GI_C|GetDifficulty _asbp_gi)
    (:Easy
      (Variables|Default|SetAmmoCount 60))
    (:Medium
      (Variables|Default|SetAmmoCount 30))
    (:Hard
      (Variables|Default|SetAmmoCount 15))))

(event Collision|EventActorBeginOverlap
  (params (OtherActor :type Actor%20Object%20Reference))
  (|CallParentFunction OtherActor) ; This node is disabled and will not be called.\nDrag off pins to build functionality.
)

(event EventTick
  (params (DeltaSeconds :type Float%20%28single-precision%29))
  (|CallParentFunction DeltaSeconds) ; This node is disabled and will not be called.\nDrag off pins to build functionality.
)

(fn ConstructionScript
  (|CallParentFunction))