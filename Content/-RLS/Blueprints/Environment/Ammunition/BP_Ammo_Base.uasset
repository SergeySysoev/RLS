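; Base ammo pickup actor that spins its mesh and grants ammo when the player character overlaps it.
; On overlap it plays the pickup sound, waits out its duration, then switches on AmmoType.
; It adds AmmoCount to that type's struct on the current weapon's AmmoComp (InClip for RL, Total otherwise).
; It calls OnAmmoChange only if the held weapon's name matches, then destroys itself.
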(event OnComponentBeginOverlap(Collision)
  (params (OverlappedComponent :type Primitive%20Component%20Object%20Reference) (OtherActor :type Actor%20Object%20Reference) (OtherComp :type Primitive%20Component%20Object%20Reference) (OtherBodyIndex :type Integer) (bFromSweep :type Boolean) (SweepResult :type Hit%20Result%20Structure%20%28by%20ref%29))
  (bind _returnvalue (Game|GetPlayerCharacter 0))
  (if (Utilities|Enum|Equal(Enum) (Utilities|GetDisplayName OtherActor) (Utilities|GetDisplayName _returnvalue))
    (bind _asbp_character (Utilities|Casting|CastToBP_Character _returnvalue))
    (bind _asbp_weapon_base (Utilities|Casting|CastToBP_Weapon_Base (Variables|/Game/-RLS/Blueprints/Character/BP_Character.BP_Character_C|GetCurrentWeapon _asbp_character)))
    (Components|Activation|Activate (Variables|Default|GetPickUpAudio) true)
    (Utilities|FlowControl|Delay (Variables|/Script/Engine.SoundBase|GetDuration (Variables|/Script/Engine.AudioComponent|GetSound (Variables|Default|GetPickUpAudio))))
    (switch Utilities|FlowControl|Switch|SwitchonE_WeaponName (Variables|Default|GetAmmoType)
      (:NewEnumerator0
        (bind _structout (Utilities|Struct|SetmembersinStruct_WeaponAmmo (Variables|/Game/-RLS/Blueprints/Components/BP_AmmoComp.BP_AmmoComp_C|GetAmmo_M16 (Variables|/Game/-RLS/Blueprints/Weapon/BP_Weapon_Base.BP_Weapon_Base_C|GetAmmoComp _asbp_weapon_base)) (+ (Variables|Default|GetAmmoCount) (.Total (Utilities|Struct|BreakStruct_WeaponAmmo (Variables|/Game/-RLS/Blueprints/Components/BP_AmmoComp.BP_AmmoComp_C|GetAmmo_M16 (Variables|/Game/-RLS/Blueprints/Weapon/BP_Weapon_Base.BP_Weapon_Base_C|GetAmmoComp _asbp_weapon_base)))))))
        (if (Utilities|Enum|Equal(Enum) (Variables|/Game/-RLS/Blueprints/Weapon/BP_Weapon_Base.BP_Weapon_Base_C|GetName (Variables|/Game/-RLS/Blueprints/Character/BP_Character.BP_Character_C|GetCurrentWeapon _asbp_character)) "M16")
          (Default|CallOnAmmoChange (Variables|/Game/-RLS/Blueprints/Weapon/BP_Weapon_Base.BP_Weapon_Base_C|GetAmmoComp _asbp_weapon_base) _structout))
        (Actor|DestroyActor))
      (:NewEnumerator1
        (bind _structout_2 (Utilities|Struct|SetmembersinStruct_WeaponAmmo (Variables|/Game/-RLS/Blueprints/Components/BP_AmmoComp.BP_AmmoComp_C|GetAmmo_AK74 (Variables|/Game/-RLS/Blueprints/Weapon/BP_Weapon_Base.BP_Weapon_Base_C|GetAmmoComp _asbp_weapon_base)) (+ (Variables|Default|GetAmmoCount) (.Total (Utilities|Struct|BreakStruct_WeaponAmmo (Variables|/Game/-RLS/Blueprints/Components/BP_AmmoComp.BP_AmmoComp_C|GetAmmo_AK74 (Variables|/Game/-RLS/Blueprints/Weapon/BP_Weapon_Base.BP_Weapon_Base_C|GetAmmoComp _asbp_weapon_base)))))))
        (if (Utilities|Enum|Equal(Enum) (Variables|/Game/-RLS/Blueprints/Weapon/BP_Weapon_Base.BP_Weapon_Base_C|GetName (Variables|/Game/-RLS/Blueprints/Character/BP_Character.BP_Character_C|GetCurrentWeapon _asbp_character)) "AK74")
          (Default|CallOnAmmoChange (Variables|/Game/-RLS/Blueprints/Weapon/BP_Weapon_Base.BP_Weapon_Base_C|GetAmmoComp _asbp_weapon_base) _structout_2))
        (Actor|DestroyActor))
      (:NewEnumerator2
        (bind _structout_3 (Utilities|Struct|SetmembersinStruct_WeaponAmmo (Variables|/Game/-RLS/Blueprints/Components/BP_AmmoComp.BP_AmmoComp_C|GetAmmo_Shotgun (Variables|/Game/-RLS/Blueprints/Weapon/BP_Weapon_Base.BP_Weapon_Base_C|GetAmmoComp _asbp_weapon_base)) (+ (Variables|Default|GetAmmoCount) (.Total (Utilities|Struct|BreakStruct_WeaponAmmo (Variables|/Game/-RLS/Blueprints/Components/BP_AmmoComp.BP_AmmoComp_C|GetAmmo_Shotgun (Variables|/Game/-RLS/Blueprints/Weapon/BP_Weapon_Base.BP_Weapon_Base_C|GetAmmoComp _asbp_weapon_base)))))))
        (if (Utilities|Enum|Equal(Enum) (Variables|/Game/-RLS/Blueprints/Weapon/BP_Weapon_Base.BP_Weapon_Base_C|GetName (Variables|/Game/-RLS/Blueprints/Character/BP_Character.BP_Character_C|GetCurrentWeapon _asbp_character)) "Shotgun")
          (Default|CallOnAmmoChange (Variables|/Game/-RLS/Blueprints/Weapon/BP_Weapon_Base.BP_Weapon_Base_C|GetAmmoComp _asbp_weapon_base) _structout_3))
        (Actor|DestroyActor))
      (:NewEnumerator3
        (bind _structout_4 (Utilities|Struct|SetmembersinStruct_WeaponAmmo (Variables|/Game/-RLS/Blueprints/Components/BP_AmmoComp.BP_AmmoComp_C|GetAmmo_RL (Variables|/Game/-RLS/Blueprints/Weapon/BP_Weapon_Base.BP_Weapon_Base_C|GetAmmoComp _asbp_weapon_base)) (+ (Variables|Default|GetAmmoCount) (.InClip (Utilities|Struct|BreakStruct_WeaponAmmo (Variables|/Game/-RLS/Blueprints/Components/BP_AmmoComp.BP_AmmoComp_C|GetAmmo_RL (Variables|/Game/-RLS/Blueprints/Weapon/BP_Weapon_Base.BP_Weapon_Base_C|GetAmmoComp _asbp_weapon_base)))))))
        (if (Utilities|Enum|Equal(Enum) (Variables|/Game/-RLS/Blueprints/Weapon/BP_Weapon_Base.BP_Weapon_Base_C|GetName (Variables|/Game/-RLS/Blueprints/Character/BP_Character.BP_Character_C|GetCurrentWeapon _asbp_character)) "GrenadeLauncher")
          (Default|CallOnAmmoChange (Variables|/Game/-RLS/Blueprints/Weapon/BP_Weapon_Base.BP_Weapon_Base_C|GetAmmoComp _asbp_weapon_base) _structout_4))
        (Actor|DestroyActor))
      (:NewEnumerator5
        (bind _structout_5 (Utilities|Struct|SetmembersinStruct_WeaponAmmo (Variables|/Game/-RLS/Blueprints/Components/BP_AmmoComp.BP_AmmoComp_C|GetAmmo_DBShotgun (Variables|/Game/-RLS/Blueprints/Weapon/BP_Weapon_Base.BP_Weapon_Base_C|GetAmmoComp _asbp_weapon_base)) (+ (Variables|Default|GetAmmoCount) (.Total (Utilities|Struct|BreakStruct_WeaponAmmo (Variables|/Game/-RLS/Blueprints/Components/BP_AmmoComp.BP_AmmoComp_C|GetAmmo_DBShotgun (Variables|/Game/-RLS/Blueprints/Weapon/BP_Weapon_Base.BP_Weapon_Base_C|GetAmmoComp _asbp_weapon_base)))))))
        (if (Utilities|Enum|Equal(Enum) (Variables|/Game/-RLS/Blueprints/Weapon/BP_Weapon_Base.BP_Weapon_Base_C|GetName (Variables|/Game/-RLS/Blueprints/Character/BP_Character.BP_Character_C|GetCurrentWeapon _asbp_character)) "DBShotgun")
          (Default|CallOnAmmoChange (Variables|/Game/-RLS/Blueprints/Weapon/BP_Weapon_Base.BP_Weapon_Base_C|GetAmmoComp _asbp_weapon_base) _structout_5))
        (Actor|DestroyActor)))))

(event EventBeginPlay)

(event Collision|EventActorBeginOverlap
  (params (OtherActor :type Actor%20Object%20Reference)))

(event EventTick
  (params (DeltaSeconds :type Float%20%28single-precision%29))
  (Transformation|AddRelativeRotation (Variables|Default|GetPickupMesh) (Math|Rotator|MakeRotator 0.0 0.0 (* DeltaSeconds 1.8e+02)) false false))

(fn ConstructionScript)

(fn CalculateNewAmmo
  (params (NewParam :type Struct%20Weapon%20Ammo%20Structure)))