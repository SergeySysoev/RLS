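; BP_PC is a player controller that toggles the game's pause menu.
; Escape or P lazily creates and caches W_PauseMenu, then drives a FlipFlop that alternates between pausing and unpausing, switching menu visibility, mouse cursor and UI-only or game-only input.
; An Unpause event runs the unpause branch directly, without advancing the FlipFlop, so the next key press can repeat the unpause branch.
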(event Custom|Unpause
  ;[1 1 1] Unpause
  (Widget|RemovefromParent (Variables|Default|GetPauseMenu))
  (Game|SetGamePaused false)
  (Variables|Default|SetbShowMouseCursor false)
  (Input|SetInputModeGameOnly self))

(event EventBeginPlay)

(event Input|KeyboardEvents|P
  (params (Key :type Key%20Structure :default "None"))
  (bind _self self)
  (:Pressed
    (Utilities|IsValid (Variables|Default|GetPauseMenu)
      (:Is%20Valid
        _)
      (:Is%20Not%20Valid
        (bind _returnvalue (UserInterface|CreateWidget "/Game/-RLS/Blueprints/Widgets/W_PauseMenu.W_PauseMenu_C"))
        (Variables|Default|SetPauseMenu _returnvalue)))
    (Utilities|FlowControl|FlipFlop
      (:A
        ;[1 1 1] Pause
        (UserInterface|Viewport|AddtoViewport (Variables|Default|GetPauseMenu) 0)
        (Game|SetGamePaused true)
        (Variables|Default|SetbShowMouseCursor true)
        (Input|SetInputModeUIOnly _self 0 "DoNotLock"))
      (:B
        ;[1 1 1] Unpause
        (Widget|RemovefromParent (Variables|Default|GetPauseMenu))
        (Game|SetGamePaused false)
        (Variables|Default|SetbShowMouseCursor false)
        (Input|SetInputModeGameOnly _self)))))

(event Input|KeyboardEvents|Escape
  (params (Key :type Key%20Structure :default "None"))
  (bind _self self)
  (:Pressed
    (Utilities|IsValid (Variables|Default|GetPauseMenu)
      (:Is%20Valid
        _)
      (:Is%20Not%20Valid
        (bind _returnvalue (UserInterface|CreateWidget "/Game/-RLS/Blueprints/Widgets/W_PauseMenu.W_PauseMenu_C"))
        (Variables|Default|SetPauseMenu _returnvalue)))
    (Utilities|FlowControl|FlipFlop
      (:A
        ;[1 1 1] Pause
        (UserInterface|Viewport|AddtoViewport (Variables|Default|GetPauseMenu) 0)
        (Game|SetGamePaused true)
        (Variables|Default|SetbShowMouseCursor true)
        (Input|SetInputModeUIOnly _self 0 "DoNotLock"))
      (:B
        ;[1 1 1] Unpause
        (Widget|RemovefromParent (Variables|Default|GetPauseMenu))
        (Game|SetGamePaused false)
        (Variables|Default|SetbShowMouseCursor false)
        (Input|SetInputModeGameOnly _self)))))

(fn ConstructionScript)