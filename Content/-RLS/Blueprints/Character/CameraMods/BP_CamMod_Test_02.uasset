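; BP_CamMod_Test_02 is a test camera modifier that shifts the view for what appears to be weapon aiming.
; As Alpha rises, it slides the camera slightly along its right vector and blends FOV toward WeaponAimFOW, leaving rotation unchanged.
; The same Alpha weights a post-process override built from a hardcoded four-component vector, while the Color node or variable is unused.
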(fn BlueprintModifyCamera
  (params (DeltaTime :type Float%20%28single-precision%29) (ViewLocation :type Vector :default "0, 0, 0") (ViewRotation :type Rotator :default "0, 0, 0") (FOV :type Float%20%28single-precision%29))
  (return (Math|Vector|Lerp(Vector) ViewLocation (+ ViewLocation (* (Math|Vector|GetRightVector ViewRotation) 12.0)) (Variables|CameraModifier|GetAlpha)) ViewRotation (Math|Float|Lerp FOV (Variables|Default|GetWeaponAimFOW) (Variables|CameraModifier|GetAlpha))))

(fn BlueprintModifyPostProcess
  (params (DeltaTime :type Float%20%28single-precision%29))
  (return (Variables|CameraModifier|GetAlpha) (Utilities|Struct|MakePostProcessSettings (Math|Vector4|MakeVector4 0.5 0.7 0.0 1.0))))