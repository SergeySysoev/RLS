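; Enemy turret that spins idly until its target-check component catches a target, then aims at the player camera and fires.
; A delayed shot loop checks visibility, then line-traces to apply point damage with muzzle effects.
; Taking damage shows a hit widget and holds the alert while a timed flag lasts.
; Vitality events update the HP widget; death triggers an explosion with radial damage, adds score and destroys the actor.
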(event OnCatchTarget(BP_TargetCheck_Component)
  ;[1 1 1] Catch/Release
  (Components|Activation|Deactivate (Variables|Default|GetLaserTraceParticle))
  (Variables|Default|SetIsTargetNear true)
  (Rendering|SetVisibility (Variables|Default|GetWidget_Alarm) true false)
  (Utilities|FlowControl|Delay 2.0)
  (CallFunction|TryMakeShot))

(event OnHPChange(BP_VitalityComponent)
  (params (CurrentHP :type Float%20%28single-precision%29) (TotalHP :type Float%20%28single-precision%29) (Hit :type Hit%20Result%20Structure) (Heal :type Boolean))
  ;[1 1 1] Update HP
  (Utilities|SetHPtoWidget CurrentHP TotalHP)
  (Variables|Default|SetGotDamage true)
  (Utilities|FlowControl|Delay (Variables|Default|GetDamageTimer))
  (Variables|Default|SetGotDamage false))

(event OnReleaseTarget(BP_TargetCheck_Component)
  (bind _weapon_root (Variables|Default|GetWeapon_Root))
  ;[1 1 1] Catch/Release
  (Components|Activation|Activate (Variables|Default|GetLaserTraceParticle) false)
  (Variables|Default|SetIsTargetNear false)
  (Rendering|SetVisibility (Variables|Default|GetWidget_Alarm) false false)
  (Transformation|SetRelativeRotation _weapon_root (Math|Rotator|MakeRotator 0.0 0.0 (.yaw (Variables|/Script/Engine.SceneComponent|GetRelativeRotation _weapon_root))) false false)
  ;;[1 1 1] Для задачи со звёздочкой
  (Transformation|SetRelativeRotation (Variables|Default|GetWeapon_Root_02) "0, 0, 0" false false))

(event OnHeal(BP_VitalityComponent)
  (params (CurrentHP :type Float%20%28single-precision%29) (TotalHP :type Float%20%28single-precision%29))
  ;[1 1 1] Update HP
  (Utilities|SetHPtoWidget CurrentHP TotalHP))

(event OnDeath(BP_VitalityComponent)
  (params (Hit :type Hit%20Result%20Structure))
  ;[1 1 1] Destroy
  (CallFunction|DestroyTurret))

(event Custom|TryMakeShot
  ;[1 1 1] Shooting
  (if (and (Variables|Default|GetIsTargetNear) (Variables|/Game/-RLS/Blueprints/Components/BP_VitalityComponent.BP_VitalityComponent_C|GetIsAlive (Variables|Default|GetBP_VitalityComponent)))
    (bind _is_visible (Default|IsVisible (Variables|Default|GetBP_TargetCheck_Component) :!label _label))
    (if _is_visible
      (Utilities|FlowControl|Sequence
        (:then_0
          (Utilities|FlowControl|Delay 3.0)
          (CallFunction|TryMakeShot))
        (:then_1
          (bind (_outhit _returnvalue) (Collision|LineTraceByChannel (Transformation|GetWorldLocation (Variables|Default|GetWeaponDir)) (- (Camera|GetCameraLocation (Game|GetPlayerCameraManager 0)) "0, 0,20.000000") "TraceTypeQuery2" true 0 "None"))
          (if _returnvalue
            (Game|Damage|ApplyPointDamage (.HitActor (Collision|BreakHitResult _outhit)) 2e+01 (Math|Vector|Normalize (- (.TraceEnd (Collision|BreakHitResult _outhit)) (.TraceStart (Collision|BreakHitResult _outhit)))) _outhit 0 self "/Game/-RLS/Blueprints/Damage/DamageType/BP_DT_M16.BP_DT_M16_C")
            (CallFunction|ActivateFireFX))))
      (else
        (Utilities|FlowControl|Delay 1.0)
        (goto _label)))))

(event Custom|DestroyTurret
  (bind _returnvalue (Transformation|GetActorLocation))
  (bind _cube2 (Variables|Default|GetCube2))
  ;[1 1 1] Destroy
  (Utilities|FlowControl|DoOnce false
    (:Completed
      (Utilities|FlowControl|Sequence
        (:then_0
          (Components|Activation|Deactivate (Variables|Default|GetBP_TargetCheck_Component))
          (Rendering|SetVisibility (Variables|Default|GetWidget_HP) false false)
          (Actor|Tick|SetActorTickEnabled false)
          (Physics|SetSimulatePhysics _cube2 true)
          (Physics|AddImpulse _cube2 "0, 0,500.000000" "None" true)
          (Class|PrimitiveComponent|AddAngularImpulseinDegrees _cube2 "30.000000,30.000000,30.000000" "None" true))
        (:then_1
          (Effects|SpawnEmitteratLocation "/Game/MilitaryWeapDark/FX/P_Grenade_Explosion_01.P_Grenade_Explosion_01" _returnvalue)
          (Audio|SpawnSoundatLocation "/Game/MilitaryWeapDark/Sound/RocketLauncher/RocketLauncher_Explosion_Cue.RocketLauncher_Explosion_Cue" _returnvalue "0, 0, 0" 1.0 1.0 0.0 0 0)
          (Rendering|Material|SetMaterial (Variables|Default|GetBase) 0 "/Game/-RLS/Materials/Turret/MI_Turret_Death.MI_Turret_Death")
          (Game|Damage|ApplyRadialDamage 2e+01 (Transformation|GetActorLocation) 5e+02 "/Game/-RLS/Blueprints/Damage/DamageType/BP_DT_GrenadeLauncher.BP_DT_GrenadeLauncher_C" 0 self 0 true "ECC_GameTraceChannel1")
          (bind _asbp_gi (Utilities|Casting|CastToBP_GI (Game|GetGameInstance)))
          (Variables|/Game/-RLS/Blueprints/Core/BP_GI.BP_GI_C|SetScore _asbp_gi (+ (Variables|/Game/-RLS/Blueprints/Core/BP_GI.BP_GI_C|GetScore _asbp_gi) (Variables|Default|GetScore_Value)))
          (Actor|DestroyActor))))))

(event EventBeginPlay
  (Components|Activation|Activate (Variables|Default|GetLaserTraceParticle) false)
  (Utilities|Casting|CastToBP_GI (Game|GetGameInstance)))

(event EventTick
  (params (DeltaSeconds :type Float%20%28single-precision%29))
  (bind _returnvalue (Game|GetPlayerCameraManager 0))
  (bind _weapon_root (Variables|Default|GetWeapon_Root))
  (bind _weapon_root_2 (Variables|Default|GetWeapon_Root))
  (bind _weapon_root_02 (Variables|Default|GetWeapon_Root_02))
  (bind _returnvalue_2 (Camera|GetCameraLocation _returnvalue))
  (Utilities|FlowControl|Sequence
    (:then_0
      (if (Variables|Default|GetIsTargetNear)
        (if true
          (Transformation|SetWorldRotation _weapon_root_2 (Math|Rotator|FindLookatRotation (Transformation|GetWorldLocation _weapon_root_2) (Camera|GetCameraLocation (Game|GetPlayerCameraManager 0))) false false)
          (else
            ;[1 1 1] Решение задачи со звёздочкой
            (Transformation|SetRelativeRotation _weapon_root (Math|Rotator|MakeRotator 0.0 0.0 (.Yaw (Math|Rotator|BreakRotator (CallFunction|FindTurretRotation (Transformation|GetWorldLocation _weapon_root) _returnvalue_2)))) false false)
            (Transformation|SetRelativeRotation _weapon_root_02 (Math|Rotator|MakeRotator 0.0 (.Pitch (Math|Rotator|BreakRotator (CallFunction|FindTurretRotation (Transformation|GetWorldLocation _weapon_root_02) _returnvalue_2))) 0.0) false false)))
        (else
          (Transformation|AddRelativeRotation (Variables|Default|GetWeapon_Root) (Math|Rotator|MakeRotator 0.0 0.0 (* DeltaSeconds 1.8e+02)) false false))))
    (:then_1
      (Transformation|SetWorldRotation (Variables|Default|GetWidget_HP) (Math|Rotator|MakeRotator 0.0 0.0 (.yaw (Math|Rotator|FindLookatRotation (Transformation|GetWorldLocation (Variables|Default|GetWidget_HP)) (Camera|GetCameraLocation (Game|GetPlayerCameraManager 0))))) false false))))

(event Game|Damage|EventAnyDamage
  (params (Damage :type Float%20%28single-precision%29) (DamageType :type Damage%20Type%20Object%20Reference) (InstigatedBy :type Controller%20Object%20Reference) (DamageCauser :type Actor%20Object%20Reference))
  (bind _bp_targetcheck_component (Variables|Default|GetBP_TargetCheck_Component))
  (bind _returnvalue (UserInterface|CreateWidget "/Game/-RLS/Blueprints/Widgets/W_Hit.W_Hit_C"))
  (UserInterface|Viewport|AddtoViewport _returnvalue 0)
  (Default|CallOnCatchTarget _bp_targetcheck_component :!label _label)
  (Utilities|FlowControl|Delay 1.0)
  (if (Variables|Default|GetGotDamage)
    (goto _label)
    (else
      (Default|CallOnReleaseTarget _bp_targetcheck_component))))

(fn ConstructionScript)

(fn FindTurretRotation
  (params (Start :type Vector%20%28by%20ref%29) (Target :type Vector%20%28by%20ref%29))
  (return (Math|Transform|InverseTransformRotation (Transformation|GetActorTransform) (Math|Rotator|FindLookatRotation Start Target))))

(fn ActivateFireFX
  (Components|Activation|Activate (Variables|Default|GetMuzzleParticle) true))