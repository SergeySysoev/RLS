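; Samurai boss enemy whose destruction ends the game: it pauses, adds its score to the game instance and shows the game over widget.
; BeginPlay caches the game instance, fills and shows the HP widget, spawns a weapon and binds the destroy handler, without calling the parent BeginPlay.
; Damage always shows a hit widget; behind a GotDamage flag, a living boss plays a random hit montage and starts hunting if idle.
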(event Custom|Game%20Finish
  (params (DestroyedActor :type Actor%20Object%20Reference))
  (Game|SetGamePaused true)
  (bind _asbp_gi (Utilities|Casting|CastToBP_GI (Game|GetGameInstance)))
  (Variables|/Game/-RLS/Blueprints/Core/BP_GI.BP_GI_C|SetScore _asbp_gi (+ (Variables|/Game/-RLS/Blueprints/Core/BP_GI.BP_GI_C|GetScore _asbp_gi) (Variables|Default|GetScore%20Value)))
  (Utilities|Casting|CastToBP_Character (Game|GetPlayerCharacter 0))
  (bind _asbp_pc (Utilities|Casting|CastToBP_PC (Game|GetPlayerController 0)))
  (bind _returnvalue (UserInterface|CreateWidget "/Game/-RLS/Blueprints/Widgets/W_GameOver.W_GameOver_C" _asbp_pc))
  (UserInterface|Viewport|AddtoViewport _returnvalue 0))

(event EventBeginPlay
  (bind _asw_hp (CallFunction|GetHPWidget))
  (bind _bp_vitalitycomponent (Variables|Default|GetBP_VitalityComponent))
  (bind _totalhp (Variables|/Game/-RLS/Blueprints/Components/BP_VitalityComponent.BP_VitalityComponent_C|GetTotalHP _bp_vitalitycomponent))
  (bind _asbp_gi (Utilities|Casting|CastToBP_GI (Game|GetGameInstance)))
  (Variables|Default|SetGame%20Instance _asbp_gi)
  (Default|SetHP _asw_hp _totalhp _totalhp)
  (Widget|SetVisibility _asw_hp "Visible")
  (CallFunction|SpawnWeapon)
  (Game|BindEventtoOnDestroyed (delegate Custom|Game%20Finish)))

(event Collision|EventActorBeginOverlap
  (params (OtherActor :type Actor%20Object%20Reference)))

(event EventTick
  (params (DeltaSeconds :type Float%20%28single-precision%29))
  (|CallParentFunction DeltaSeconds) ; This node is disabled and will not be called.\nDrag off pins to build functionality.
)

(event EventAnyDamage
  (params (Damage :type Float%20%28single-precision%29) (DamageType :type Damage%20Type%20Object%20Reference) (InstigatedBy :type Controller%20Object%20Reference) (DamageCauser :type Actor%20Object%20Reference))
  (bind _hit_montage (Variables|Default|GetHit_Montage))
  (bind _returnvalue (UserInterface|CreateWidget "/Game/-RLS/Blueprints/Widgets/W_Hit.W_Hit_C"))
  (UserInterface|Viewport|AddtoViewport _returnvalue 0)
  (if (not (Variables|Default|GetGotDamage))
    (Variables|Default|SetGotDamage true)
    (if (Variables|/Game/-RLS/Blueprints/Components/BP_VitalityComponent.BP_VitalityComponent_C|GetIsAlive (Variables|Default|GetBP_VitalityComponent))
      (Animation|Montage|PlayMontage (Variables|Character|GetMesh) (Utilities|Array|Get(acopy) _hit_montage (Math|Random|RandomInteger (Utilities|Array|Length _hit_montage)))
        (:then
          (if (not (Variables|Default|GetIsHunting))
            (CallFunction|StartHunt)))))))

(fn ConstructionScript
  (|CallParentFunction))