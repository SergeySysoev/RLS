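; BP_EW_ArachnidLeg is an enemy melee weapon, named for an arachnid leg, that deals point damage through a box hitbox.
; ActivateDamageCollision toggles the box between query-only and no collision, clearing the list of damaged actors each time.
; On overlap, an actor not yet in that list is recorded and damaged using the sweep result, limiting it to one hit per activation.
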(event OnComponentBeginOverlap(Box)
  (params (OverlappedComponent :type Primitive%20Component%20Object%20Reference) (OtherActor :type Actor%20Object%20Reference) (OtherComp :type Primitive%20Component%20Object%20Reference) (OtherBodyIndex :type Integer) (bFromSweep :type Boolean) (SweepResult :type Hit%20Result%20Structure%20%28by%20ref%29))
  (bind _damagedactorsarr (Variables|Default|GetDamagedActorsArr))
  (if (not (Utilities|Array|ContainsItem _damagedactorsarr OtherActor))
    (Utilities|Array|AddUnique _damagedactorsarr OtherActor)
    (Game|Damage|ApplyPointDamage OtherActor (Variables|Default|GetDamage) (Math|Vector|MakeVector 0.0 0.0 0.0) SweepResult 0 self (Variables|Default|GetDamageType))))

(event Custom|ActivateDamageCollision
  (params (OnOff :type Boolean))
  (Collision|SetCollisionEnabled (Variables|Default|GetBox) (select OnOff "QueryOnly" "NoCollision"))
  (Utilities|Array|Clear (Variables|Default|GetDamagedActorsArr)))

(event EventBeginPlay)

(event Collision|EventActorBeginOverlap
  (params (OtherActor :type Actor%20Object%20Reference)))

(event EventTick
  (params (DeltaSeconds :type Float%20%28single-precision%29)))

(fn ConstructionScript)