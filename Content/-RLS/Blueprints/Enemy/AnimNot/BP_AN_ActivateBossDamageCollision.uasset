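; Anim notify state that opens a damage window on a boss's weapon during an animation.
; On begin it casts the mesh owner to OUTDATED_BP_Boss_Base and turns on damage collision on its current weapon; on end it turns that collision off.
; Owners that are not that outdated boss base class are ignored.
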(fn ReceivedNotifyBegin
  (params (MeshComp :type Skeletal%20Mesh%20Component%20Object%20Reference) (Animation :type Anim%20Sequence%20Base%20Object%20Reference) (TotalDuration :type Float%20%28single-precision%29))
  (bind _asbp_boss_base (Utilities|Casting|CastToOUTDATED_BP_Boss_Base (Components|GetOwner MeshComp)))
  (Default|ActivateDamageCollision (Variables|/Game/-RLS/Blueprints/Enemy/OUTDATED_BP_Boss_Base.OUTDATED_BP_Boss_Base_C|GetCurrentWeapon _asbp_boss_base) true)
  (return false))

(fn ReceivedNotifyEnd
  (params (MeshComp :type Skeletal%20Mesh%20Component%20Object%20Reference) (Animation :type Anim%20Sequence%20Base%20Object%20Reference))
  (bind _asbp_boss_base (Utilities|Casting|CastToOUTDATED_BP_Boss_Base (Components|GetOwner MeshComp)))
  (Default|ActivateDamageCollision (Variables|/Game/-RLS/Blueprints/Enemy/OUTDATED_BP_Boss_Base.OUTDATED_BP_Boss_Base_C|GetCurrentWeapon _asbp_boss_base) false)
  (return true))