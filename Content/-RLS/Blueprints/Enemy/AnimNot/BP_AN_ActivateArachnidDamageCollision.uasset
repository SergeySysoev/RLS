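; Anim notify state that opens and closes damage collision windows on BP_ArachnidBoss limbs during its four attack animations.
; It switches on the animation's display name, casts the mesh owner to the boss, then toggles the left claw, right claw, both claws or both legs.
; Notify begin matches names ending in "Montage", while notify end matches the same attack names without that suffix.
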(fn ReceivedNotifyBegin
  (params (MeshComp :type Skeletal%20Mesh%20Component%20Object%20Reference) (Animation :type Anim%20Sequence%20Base%20Object%20Reference) (TotalDuration :type Float%20%28single-precision%29))
  (bind _returnvalue (Components|GetOwner MeshComp))
  (switch string (Utilities|GetDisplayName Animation)
    (:Anim_Arachnid_Boss_Attack_1_Montage
      (bind _asbp_arachnid_boss (Utilities|Casting|CastToBP_ArachnidBoss _returnvalue))
      (Default|ActivateDamageCollision (Variables|/Game/-RLS/Blueprints/Enemy/BP_ArachnidBoss.BP_ArachnidBoss_C|GetLeftClaw _asbp_arachnid_boss) true))
    (:Anim_Arachnid_Boss_Attack_2_Montage
      (bind _asbp_arachnid_boss_2 (Utilities|Casting|CastToBP_ArachnidBoss _returnvalue))
      (Default|ActivateDamageCollision (Variables|/Game/-RLS/Blueprints/Enemy/BP_ArachnidBoss.BP_ArachnidBoss_C|GetRightClaw _asbp_arachnid_boss_2) true))
    (:Anim_Arachnid_Boss_Attack_3_Montage
      (bind _asbp_arachnid_boss_3 (Utilities|Casting|CastToBP_ArachnidBoss _returnvalue))
      (Default|ActivateDamageCollision (Variables|/Game/-RLS/Blueprints/Enemy/BP_ArachnidBoss.BP_ArachnidBoss_C|GetRightClaw _asbp_arachnid_boss_3) true)
      (Default|ActivateDamageCollision (Variables|/Game/-RLS/Blueprints/Enemy/BP_ArachnidBoss.BP_ArachnidBoss_C|GetLeftClaw _asbp_arachnid_boss_3) true))
    (:Anim_Arachnid_Boss_Attack_4_Montage
      (bind _asbp_arachnid_boss_4 (Utilities|Casting|CastToBP_ArachnidBoss _returnvalue))
      (Default|ActivateDamageCollision (Variables|/Game/-RLS/Blueprints/Enemy/BP_ArachnidBoss.BP_ArachnidBoss_C|GetRightLeg _asbp_arachnid_boss_4) true)
      (Default|ActivateDamageCollision (Variables|/Game/-RLS/Blueprints/Enemy/BP_ArachnidBoss.BP_ArachnidBoss_C|GetLeftLeg _asbp_arachnid_boss_4) true)))
  (return false))

(fn ReceivedNotifyEnd
  (params (MeshComp :type Skeletal%20Mesh%20Component%20Object%20Reference) (Animation :type Anim%20Sequence%20Base%20Object%20Reference))
  (bind _returnvalue (Components|GetOwner MeshComp))
  (switch string (Utilities|GetDisplayName Animation)
    (:Anim_Arachnid_Boss_Attack_1
      (bind _asbp_arachnid_boss (Utilities|Casting|CastToBP_ArachnidBoss _returnvalue))
      (Default|ActivateDamageCollision (Variables|/Game/-RLS/Blueprints/Enemy/BP_ArachnidBoss.BP_ArachnidBoss_C|GetLeftClaw _asbp_arachnid_boss) false))
    (:Anim_Arachnid_Boss_Attack_2
      (bind _asbp_arachnid_boss_2 (Utilities|Casting|CastToBP_ArachnidBoss _returnvalue))
      (Default|ActivateDamageCollision (Variables|/Game/-RLS/Blueprints/Enemy/BP_ArachnidBoss.BP_ArachnidBoss_C|GetRightClaw _asbp_arachnid_boss_2) false))
    (:Anim_Arachnid_Boss_Attack_3
      (bind _asbp_arachnid_boss_3 (Utilities|Casting|CastToBP_ArachnidBoss _returnvalue))
      (Default|ActivateDamageCollision (Variables|/Game/-RLS/Blueprints/Enemy/BP_ArachnidBoss.BP_ArachnidBoss_C|GetRightClaw _asbp_arachnid_boss_3) false)
      (Default|ActivateDamageCollision (Variables|/Game/-RLS/Blueprints/Enemy/BP_ArachnidBoss.BP_ArachnidBoss_C|GetLeftClaw _asbp_arachnid_boss_3) false))
    (:Anim_Arachnid_Boss_Attack_4
      (bind _asbp_arachnid_boss_4 (Utilities|Casting|CastToBP_ArachnidBoss _returnvalue))
      (Default|ActivateDamageCollision (Variables|/Game/-RLS/Blueprints/Enemy/BP_ArachnidBoss.BP_ArachnidBoss_C|GetRightLeg _asbp_arachnid_boss_4) false)
      (Default|ActivateDamageCollision (Variables|/Game/-RLS/Blueprints/Enemy/BP_ArachnidBoss.BP_ArachnidBoss_C|GetLeftLeg _asbp_arachnid_boss_4) false)))
  (return true))