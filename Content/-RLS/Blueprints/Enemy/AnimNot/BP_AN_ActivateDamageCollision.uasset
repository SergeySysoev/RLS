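; Anim notify state that toggles damage collision on an enemy's current weapon during an animation window.
; Begin and end each cast the mesh owner to BP_Enemy_Base, falling back to BP_BTEnemy_Base, then call ActivateDamageCollision on CurrentWeapon.
; BP_Enemy_Base weapons switch on at begin and off at end.
; BP_BTEnemy_Base weapons receive false at both, so this notify never enables their collision.
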(fn ReceivedNotifyBegin
  (params (MeshComp :type Skeletal%20Mesh%20Component%20Object%20Reference) (Animation :type Anim%20Sequence%20Base%20Object%20Reference) (TotalDuration :type Float%20%28single-precision%29))
  (bind _returnvalue (Components|GetOwner MeshComp))
  (bind _asbp_enemy_base (Utilities|Casting|CastToBP_Enemy_Base _returnvalue)
    (:then
      (Default|ActivateDamageCollision (Variables|/Game/-RLS/Blueprints/Enemy/BP_Enemy_Base.BP_Enemy_Base_C|GetCurrentWeapon _asbp_enemy_base) true)
      (return false))
    (:CastFailed
      (bind _asbp_btenemy_base (Utilities|Casting|CastToBP_BTEnemy_Base _returnvalue))
      (Default|ActivateDamageCollision (Variables|/Game/-RLS/Blueprints/Enemy/BehaviourTree/BP_BTEnemy_Base.BP_BTEnemy_Base_C|GetCurrent%20Weapon _asbp_btenemy_base) false)
      (return false))))

(fn ReceivedNotifyEnd
  (params (MeshComp :type Skeletal%20Mesh%20Component%20Object%20Reference) (Animation :type Anim%20Sequence%20Base%20Object%20Reference))
  (bind _returnvalue (Components|GetOwner MeshComp))
  (bind _asbp_enemy_base (Utilities|Casting|CastToBP_Enemy_Base _returnvalue)
    (:then
      (Default|ActivateDamageCollision (Variables|/Game/-RLS/Blueprints/Enemy/BP_Enemy_Base.BP_Enemy_Base_C|GetCurrentWeapon _asbp_enemy_base) false)
      (return true))
    (:CastFailed
      (bind _asbp_btenemy_base (Utilities|Casting|CastToBP_BTEnemy_Base _returnvalue))
      (Default|ActivateDamageCollision (Variables|/Game/-RLS/Blueprints/Enemy/BehaviourTree/BP_BTEnemy_Base.BP_BTEnemy_Base_C|GetCurrent%20Weapon _asbp_btenemy_base) false)
      (return true))))