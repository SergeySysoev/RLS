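; Base enemy character that hunts and attacks the player, with weapon, health and detection range set up on spawn from BP_GI difficulty settings.
; Target-check catch or damage starts a hunt: AIMoveTo the player, random attack montage, reaction delay, repeating while alive without checking IsHunting.
; Damage shows hit feedback, with blood and montages.
; Vitality component events update the HP widget and handle death: weapon removal, ragdoll, delayed destruction and score award.
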(event OnHPChange(BP_VitalityComponent)
  (params (CurrentHP :type Float%20%28single-precision%29) (TotalHP :type Float%20%28single-precision%29) (Hit :type Hit%20Result%20Structure) (Heal :type Boolean))
  ;[1 1 1] Vitality
  (Default|SetHP (CallFunction|GetHPWidget) CurrentHP TotalHP))

(event OnDeath(BP_VitalityComponent)
  (params (Hit :type Hit%20Result%20Structure))
  (bind _mesh (Variables|Character|GetMesh))
  ;[1 1 1] Death
  (Utilities|FlowControl|Sequence
    (:then_0
      (Actor|DestroyActor (Variables|Default|GetCurrentWeapon)))
    (:then_1
      (Collision|SetCollisionProfileName _mesh "PhysicsActor" true :!class /Script/Engine.PrimitiveComponent)
      (Physics|SetSimulatePhysics _mesh true)
      (Collision|SetCollisionEnabled (Variables|Collision|GetCapsuleComponent) "NoCollision")
      (Rendering|SetVisibility (Variables|Components|GetWidget_HP) false false))
    (:then_2
      (Utilities|FlowControl|Delay 1.0)
      (Actor|DestroyActor)
      (bind _asbp_gi (Utilities|Casting|CastToBP_GI (Game|GetGameInstance)))
      (Variables|/Game/-RLS/Blueprints/Core/BP_GI.BP_GI_C|SetScore _asbp_gi (+ (Variables|/Game/-RLS/Blueprints/Core/BP_GI.BP_GI_C|GetScore _asbp_gi) (Variables|Default|GetScore%20Value))))))

(event OnCatchTarget(BP_TargetCheck_Component)
  ;[1 1 1] Cheking for the Player
  (Variables|Default|SetIsTargetNear true)
  (CallFunction|StartHunt))

(event OnReleaseTarget(BP_TargetCheck_Component)
  ;[1 1 1] Cheking for the Player
  (Variables|Default|SetIsTargetNear false)
  (CallFunction|StopHunt))

(event Custom|StartHunt
  ;[1 1 1] Hunt
  (Variables|Default|SetIsHunting true)
  (Audio|Components|Audio|Play (Variables|Components|GetHunt%20Scream) 0.0)
  (CallFunction|HuntIteration))

(event Custom|Hunt%20Iteration
  (bind _capsulecomponent (Variables|Collision|GetCapsuleComponent))
  (bind _attack_montage (Variables|-Montages|GetAttack_Montage))
  (bind _returnvalue (Utilities|Array|Length _attack_montage))
  (bind _returnvalue_2 (Math|Random|RandomInteger _returnvalue))
  (bind _output (Utilities|Array|Get(acopy) _attack_montage _returnvalue_2))
  ;[1 1 1] Hunt
  (if (Variables|/Game/-RLS/Blueprints/Components/BP_VitalityComponent.BP_VitalityComponent_C|GetIsAlive (Variables|Components|GetBP_VitalityComponent))
    (bind _movementresult (AI|AIMoveTo self "0, 0, 0" (Game|GetPlayerCharacter 0) 2e+02 true)
      (:OnSuccess
        (Transformation|SetWorldRotation _capsulecomponent (Math|Rotator|MakeRotator 0.0 0.0 (Math|Float|Lerp (.yaw (Transformation|GetWorldRotation _capsulecomponent)) (.yaw (Math|Rotator|FindLookatRotation (Transformation|GetWorldLocation _capsulecomponent) (Camera|GetCameraLocation (Game|GetPlayerCameraManager 0)))) 1.0)) false false)
        (Development|PrintString "go to montage")
        (Animation|Montage|PlayMontage (Variables|Character|GetMesh) _output
          (:OnCompleted
            (Animation|StopAnimMontage _output))
          (:OnInterrupted
            _))
        (CallFunction|HuntWait)))))

(event Custom|Hunt_Wait
  ;[1 1 1] Hunt
  (Utilities|FlowControl|Delay (Variables|/Game/-RLS/Blueprints/Core/BP_GI.BP_GI_C|GetEnemy_Reaction_Time (Variables|Default|GetGame%20Instance)))
  (CallFunction|HuntIteration))

(event Custom|Footstep_Event
  ;[1 1 1] Footsteps Sound
  (Audio|Components|Audio|Play (Variables|Components|GetFootstep) 0.0))

(event Custom|Stop%20Hunt
  ;[1 1 1] Hunt
  (Variables|Default|SetIsHunting false))

(event Custom|StopAttack
  ;[1 1 1] Hunt
)

(event EventBeginPlay
  (bind _bp_targetcheck_component (Variables|Components|GetBP_TargetCheck_Component))
  ;[1 1 1] Begin Play: Set Weapon, HP, Catch/Release Distance
  (CallFunction|SpawnWeapon)
  (|SetEnemyHPaccordingtothedifficultysettings)
  (bind _asbp_gi (Utilities|Casting|CastToBP_GI (Game|GetGameInstance)))
  (Variables|/Game/-RLS/Blueprints/Components/BP_TargetCheck_Component.BP_TargetCheck_Component_C|SetCatch_Distance _bp_targetcheck_component (Variables|/Game/-RLS/Blueprints/Core/BP_GI.BP_GI_C|GetEnemy_Catch_Distance _asbp_gi))
  (Variables|/Game/-RLS/Blueprints/Components/BP_TargetCheck_Component.BP_TargetCheck_Component_C|SetRelease_Distance _bp_targetcheck_component (Variables|/Game/-RLS/Blueprints/Core/BP_GI.BP_GI_C|GetEnemy_Release_Distance _asbp_gi)))

(event EventTick
  (params (DeltaSeconds :type Float%20%28single-precision%29))
  ;[1 1 1] Cheking for the Player
)

(event Game|Damage|EventPointDamage
  (params (Damage :type Float%20%28single-precision%29) (DamageType :type Damage%20Type%20Object%20Reference) (HitLocation :type Vector :default "0, 0, 0") (HitNormal :type Vector :default "0, 0, 0") (HitComponent :type Primitive%20Component%20Object%20Reference) (BoneName :type Name :default "None") (ShotFromDirection :type Vector :default "0, 0, 0") (InstigatedBy :type Controller%20Object%20Reference) (DamageCauser :type Actor%20Object%20Reference) (HitInfo :type Hit%20Result%20Structure%20%28by%20ref%29))
  (bind _hit_montage (Variables|-Montages|GetHit_Montage))
  ;[1 1 1] Got Damage
  (Effects|SpawnEmitteratLocation "/Game/BallisticsVFX/Particles/Impacts/DynamicImpacts/Flesh/Blood_cloud_Dyn_2.Blood_cloud_Dyn_2" HitLocation (Math|Conversions|RotationFromXVector (* ShotFromDirection -1)))
  (bind _returnvalue (UserInterface|CreateWidget "/Game/-RLS/Blueprints/Widgets/W_Hit.W_Hit_C"))
  (UserInterface|Viewport|AddtoViewport _returnvalue 0)
  (if (Utilities|Name|Equal(Name) BoneName "head")
    (Variables|Default|SetGotDamage false))
  (if (not (Variables|Default|GetGotDamage))
    (Variables|Default|SetGotDamage true)
    (if (Variables|/Game/-RLS/Blueprints/Components/BP_VitalityComponent.BP_VitalityComponent_C|GetIsAlive (Variables|Components|GetBP_VitalityComponent))
      (Animation|Montage|PlayMontage (Variables|Character|GetMesh) (Utilities|Array|Get(acopy) _hit_montage (Math|Random|RandomInteger (Utilities|Array|Length _hit_montage)))
        (:then
          (if (not (Variables|Default|GetIsHunting))
            (CallFunction|StartHunt)))))))

(event Game|Damage|EventAnyDamage
  (params (Damage :type Float%20%28single-precision%29) (DamageType :type Damage%20Type%20Object%20Reference) (InstigatedBy :type Controller%20Object%20Reference) (DamageCauser :type Actor%20Object%20Reference))
  (bind _hit_montage (Variables|-Montages|GetHit_Montage))
  ;[1 1 1] Got Damage
  (Effects|SpawnEmitteratLocation "/Game/BallisticsVFX/Particles/Impacts/DynamicImpacts/Flesh/Blood_cloud_Dyn_2.Blood_cloud_Dyn_2" (stale Game|Damage|EventPointDamage HitLocation) (Math|Conversions|RotationFromXVector (* (stale Game|Damage|EventPointDamage ShotFromDirection) -1)))
  (bind _returnvalue (UserInterface|CreateWidget "/Game/-RLS/Blueprints/Widgets/W_Hit.W_Hit_C"))
  (UserInterface|Viewport|AddtoViewport _returnvalue 0)
  (if (Utilities|Name|Equal(Name) (stale Game|Damage|EventPointDamage BoneName) "head")
    (Variables|Default|SetGotDamage false))
  (if (not (Variables|Default|GetGotDamage))
    (Variables|Default|SetGotDamage true)
    (if (Variables|/Game/-RLS/Blueprints/Components/BP_VitalityComponent.BP_VitalityComponent_C|GetIsAlive (Variables|Components|GetBP_VitalityComponent))
      (Animation|Montage|PlayMontage (Variables|Character|GetMesh) (Utilities|Array|Get(acopy) _hit_montage (Math|Random|RandomInteger (Utilities|Array|Length _hit_montage)))
        (:then
          (if (not (Variables|Default|GetIsHunting))
            (CallFunction|StartHunt)))))))

(event Game|Damage|EventRadialDamage
  (params (DamageReceived :type Float%20%28single-precision%29) (DamageType :type Damage%20Type%20Object%20Reference) (Origin :type Vector :default "0, 0, 0") (HitInfo :type Hit%20Result%20Structure%20%28by%20ref%29) (InstigatedBy :type Controller%20Object%20Reference) (DamageCauser :type Actor%20Object%20Reference))
  (bind _hit_montage (Variables|-Montages|GetHit_Montage))
  ;[1 1 1] Got Damage
  (bind _returnvalue (UserInterface|CreateWidget "/Game/-RLS/Blueprints/Widgets/W_Hit.W_Hit_C"))
  (UserInterface|Viewport|AddtoViewport _returnvalue 0)
  (if (Utilities|Name|Equal(Name) (stale Game|Damage|EventPointDamage BoneName) "head")
    (Variables|Default|SetGotDamage false))
  (if (not (Variables|Default|GetGotDamage))
    (Variables|Default|SetGotDamage true)
    (if (Variables|/Game/-RLS/Blueprints/Components/BP_VitalityComponent.BP_VitalityComponent_C|GetIsAlive (Variables|Components|GetBP_VitalityComponent))
      (Animation|Montage|PlayMontage (Variables|Character|GetMesh) (Utilities|Array|Get(acopy) _hit_montage (Math|Random|RandomInteger (Utilities|Array|Length _hit_montage)))
        (:then
          (if (not (Variables|Default|GetIsHunting))
            (CallFunction|StartHunt)))))))

(fn ConstructionScript)

(fn SpawnWeapon
  (bind _returnvalue (Game|SpawnActorfromClass (Variables|Default|GetWeaponClass) (Math|Transform|MakeTransform "0, 0, 0" "0, 0, 0" "1,1,1") "AlwaysSpawn" 0 0))
  (bind _output_get (Variables|Default|SetCurrentWeapon _returnvalue))
  (Transformation|AttachComponentToComponent _output_get (Variables|Character|GetMesh) "Hand_RSocket" "SnapToTarget" "SnapToTarget" "SnapToTarget" true))

(fn GetHPWidget
  (bind _asw_hp (Utilities|Casting|CastToW_HP (UserInterface|GetUserWidgetObject (Variables|Components|GetWidget_HP))))
  (return _asw_hp))