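; Base behavior-tree enemy Blueprint with a vitality component, HP widget, status particle effect and footstep sound.
; BeginPlay caches the AI controller and game instance, then scales HP by the game instance's enemy health multiplier.
; Any, point and radial damage set the GotDamage blackboard flag, while vitality HP changes refresh the widget.
; Blood, hit-widget and hit-montage reaction logic is present but disconnected.
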(event OnHPChange(BP_VitalityComponent)
  (params (CurrentHP :type Float%20%28single-precision%29) (TotalHP :type Float%20%28single-precision%29) (Hit :type Hit%20Result%20Structure) (Heal :type Boolean))
  ;[1 1 1] Vitality
  (Default|SetHP (CallFunction|GetWidgetHP) CurrentHP TotalHP))

(event Custom|UpdateStatus
  (params (Status :type Enum_GoodParticleStatus%20Enum :default "NewEnumerator2"))
  (bind _bp_goodparticlestatus (Variables|Default|GetBP_GoodParticleStatus))
  ;[1 1 1] Change GoodParticle Effect
  (Variables|/Game/GoodParticleStatus/Blueprint/BP_GoodParticleStatus.BP_GoodParticleStatus_C|SetEffects%20Style _bp_goodparticlestatus Status)
  (Default|GoodParticleStatusUpdate _bp_goodparticlestatus))

(event Custom|Footstep_Event
  ;[1 1 1] Footsteps sound
  (Audio|Components|Audio|Play (Variables|Default|GetFootstep) 0.0))

(event EventBeginPlay
  (bind _widget_hp (CallFunction|GetWidgetHP))
  (bind _bp_vitalitycomponent (Variables|Default|GetBP_VitalityComponent))
  (bind _asbp_enemy_aic (Utilities|Casting|CastToBP_Enemy_AIC (AI|GetAIController self)))
  (Variables|Default|SetAIController _asbp_enemy_aic)
  (bind _asbp_gi (Utilities|Casting|CastToBP_GI (Game|GetGameInstance)))
  (Variables|Default|SetGame%20Instance _asbp_gi)
  (bind _output_get (Variables|/Game/-RLS/Blueprints/Components/BP_VitalityComponent.BP_VitalityComponent_C|SetCurrentHP _bp_vitalitycomponent (* (Variables|/Game/-RLS/Blueprints/Core/BP_GI.BP_GI_C|GetEnemyHealthMultiplier _asbp_gi) (Variables|/Game/-RLS/Blueprints/Components/BP_VitalityComponent.BP_VitalityComponent_C|GetTotalHP _bp_vitalitycomponent))))
  (bind _output_get_2 (Variables|/Game/-RLS/Blueprints/Components/BP_VitalityComponent.BP_VitalityComponent_C|SetTotalHP _bp_vitalitycomponent (* (Variables|/Game/-RLS/Blueprints/Core/BP_GI.BP_GI_C|GetEnemyHealthMultiplier _asbp_gi) (Variables|/Game/-RLS/Blueprints/Components/BP_VitalityComponent.BP_VitalityComponent_C|GetTotalHP _bp_vitalitycomponent))))
  (Default|SetHP _widget_hp _output_get _output_get_2)
  (Widget|SetVisibility _widget_hp "Visible"))

(event EventTick
  (params (DeltaSeconds :type Float%20%28single-precision%29)))

(event Game|Damage|EventPointDamage
  (params (Damage :type Float%20%28single-precision%29) (DamageType :type Damage%20Type%20Object%20Reference) (HitLocation :type Vector :default "0, 0, 0") (HitNormal :type Vector :default "0, 0, 0") (HitComponent :type Primitive%20Component%20Object%20Reference) (BoneName :type Name :default "None") (ShotFromDirection :type Vector :default "0, 0, 0") (InstigatedBy :type Controller%20Object%20Reference) (DamageCauser :type Actor%20Object%20Reference) (HitInfo :type Hit%20Result%20Structure%20%28by%20ref%29))
  ;[1 1 1] Got Damage
  (AI|Components|Blackboard|SetValueasBool (Variables|/Script/AIModule.AIController|GetBlackboard (Variables|Default|GetAIController)) (Utilities|Name|MakeLiteralName "GotDamage") true))

(event Game|Damage|EventAnyDamage
  (params (Damage :type Float%20%28single-precision%29) (DamageType :type Damage%20Type%20Object%20Reference) (InstigatedBy :type Controller%20Object%20Reference) (DamageCauser :type Actor%20Object%20Reference))
  ;[1 1 1] Got Damage
  (AI|Components|Blackboard|SetValueasBool (Variables|/Script/AIModule.AIController|GetBlackboard (Variables|Default|GetAIController)) (Utilities|Name|MakeLiteralName "GotDamage") true))

(event Game|Damage|EventRadialDamage
  (params (DamageReceived :type Float%20%28single-precision%29) (DamageType :type Damage%20Type%20Object%20Reference) (Origin :type Vector :default "0, 0, 0") (HitInfo :type Hit%20Result%20Structure%20%28by%20ref%29) (InstigatedBy :type Controller%20Object%20Reference) (DamageCauser :type Actor%20Object%20Reference))
  ;[1 1 1] Got Damage
  (AI|Components|Blackboard|SetValueasBool (Variables|/Script/AIModule.AIController|GetBlackboard (Variables|Default|GetAIController)) (Utilities|Name|MakeLiteralName "GotDamage") true))

(fn ConstructionScript)

(fn GetWidgetHP
  (bind _asw_hp (Utilities|Casting|CastToW_HP (UserInterface|GetUserWidgetObject (Variables|Default|GetWidget_HP))))
  (return _asw_hp))