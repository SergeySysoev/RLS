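; Arachnid boss enemy with an HP widget that spawns four weapon legs on its mesh sockets.
; Target detection or a damage reaction starts a hunt loop that moves to the player, turns and plays random attack montages.
; Hits show a hit widget, with montage reactions gated by a flag that one specific bone resets.
; Death ragdolls and destroys it, adding score, while destruction pauses the game, adds score again and shows the game-over screen.
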(event OnCatchTarget(BP_TargetCheck_Component)
  ;[1 1 1] On Target
  (Variables|Default|SetisTargetNear true)
  (CallFunction|StartHunt))

(event OnReleaseTarget(BP_TargetCheck_Component)
  ;[1 1 1] On Target
  (Variables|Default|SetisTargetNear false)
  (CallFunction|StopHunt))

(event OnHPChange(BP_VitalityComponent)
  (params (CurrentHP :type Float%20%28single-precision%29) (TotalHP :type Float%20%28single-precision%29) (Hit :type Hit%20Result%20Structure) (Heal :type Boolean))
  ;[1 1 1] Vitality
  (Default|SetHP (CallFunction|GetHPWidget) CurrentHP TotalHP))

(event OnDeath(BP_VitalityComponent)
  (params (Hit :type Hit%20Result%20Structure))
  (bind _mesh (Variables|Character|GetMesh))
  ;[1 1 1] On Death
  (Utilities|FlowControl|Sequence
    (:then_0
      (Collision|SetCollisionProfileName _mesh "PhysicsActor" true :!class /Script/Engine.PrimitiveComponent)
      (Physics|SetSimulatePhysics _mesh true)
      (Collision|SetCollisionEnabled (Variables|Collision|GetCapsuleComponent) "NoCollision")
      (Rendering|SetVisibility (Variables|Components|GetWidget_HP) false false))
    (:then_1
      (Utilities|FlowControl|Delay 1.0)
      (Actor|DestroyActor)
      (bind _asbp_gi (Utilities|Casting|CastToBP_GI (Game|GetGameInstance)))
      (Variables|/Game/-RLS/Blueprints/Core/BP_GI.BP_GI_C|SetScore _asbp_gi (+ (Variables|/Game/-RLS/Blueprints/Core/BP_GI.BP_GI_C|GetScore _asbp_gi) (Variables|Default|GetScoreValue))))))

(event OnComponentBeginOverlap(Mesh)
  (params (OverlappedComponent :type Primitive%20Component%20Object%20Reference) (OtherActor :type Actor%20Object%20Reference) (OtherComp :type Primitive%20Component%20Object%20Reference) (OtherBodyIndex :type Integer) (bFromSweep :type Boolean) (SweepResult :type Hit%20Result%20Structure%20%28by%20ref%29)))

(event Custom|StartHunt
  ;[1 1 1] Hunt
  (Variables|Default|SetIsHunting true)
  (Audio|Components|Audio|Play (Variables|Default|GetHuntScream) 0.0)
  (CallFunction|HuntIteration))

(event Custom|Hunt%20Iteration
  (bind _capsulecomponent (Variables|Collision|GetCapsuleComponent))
  (bind _attack_montage (Variables|Default|GetAttack_Montage))
  (bind _returnvalue (Utilities|Array|Length _attack_montage))
  (bind _returnvalue_2 (Math|Random|RandomInteger _returnvalue))
  (bind _output (Utilities|Array|Get(acopy) _attack_montage _returnvalue_2))
  ;[1 1 1] Hunt
  (if (Variables|/Game/-RLS/Blueprints/Components/BP_VitalityComponent.BP_VitalityComponent_C|GetIsAlive (Variables|Default|GetBP_VitalityComponent))
    (AI|AIMoveTo self "0, 0, 0" (Game|GetPlayerCharacter 0) 2.3e+02 true
      (:OnSuccess
        (Transformation|SetWorldRotation _capsulecomponent (Math|Rotator|MakeRotator 0.0 0.0 (Math|Float|Lerp (.yaw (Transformation|GetWorldRotation _capsulecomponent)) (.yaw (Math|Rotator|FindLookatRotation (Transformation|GetWorldLocation _capsulecomponent) (Camera|GetCameraLocation (Game|GetPlayerCameraManager 0)))) 1.0)) false false)
        (Animation|Montage|PlayMontage (Variables|Character|GetMesh) _output
          (:OnCompleted
            _)
          (:OnInterrupted
            _))
        (Animation|StopAnimMontage _output)
        (CallFunction|HuntWait)))))

(event Custom|Hunt_Wait
  ;[1 1 1] Hunt
  (Utilities|FlowControl|Delay 0.1)
  (CallFunction|HuntIteration))

(event Custom|Event_Footsteps
  (Audio|Components|Audio|Play (Variables|Default|GetFootstep) 0.0))

(event Custom|Stop%20Hunt
  ;[1 1 1] Hunt
  (Variables|Default|SetIsHunting false))

(event Custom|GameFinish
  (params (DestroyedActor :type Actor%20Object%20Reference))
  (Game|SetGamePaused true)
  (bind _asbp_gi (Utilities|Casting|CastToBP_GI (Game|GetGameInstance)))
  (Variables|/Game/-RLS/Blueprints/Core/BP_GI.BP_GI_C|SetScore _asbp_gi (+ (Variables|/Game/-RLS/Blueprints/Core/BP_GI.BP_GI_C|GetScore _asbp_gi) (Variables|Default|GetScoreValue)))
  (Utilities|Casting|CastToBP_Character (Game|GetPlayerCharacter 0))
  (bind _asbp_pc (Utilities|Casting|CastToBP_PC (Game|GetPlayerController 0)))
  (bind _returnvalue (UserInterface|CreateWidget "/Game/-RLS/Blueprints/Widgets/W_GameOver.W_GameOver_C" _asbp_pc))
  (UserInterface|Viewport|AddtoViewport _returnvalue 0))

(event EventBeginPlay
  (bind _hp_widget (CallFunction|GetHPWidget))
  (bind _asbp_gi (Utilities|Casting|CastToBP_GI (Game|GetGameInstance)))
  (Variables|Default|SetGame%20Instance _asbp_gi)
  (Default|SetHP _hp_widget 0.0 0.0)
  (Widget|SetVisibility _hp_widget "Visible")
  (Game|BindEventtoOnDestroyed (delegate Custom|GameFinish))
  (CallFunction|SpawnWeaponLegs))

(event Game|Damage|EventPointDamage
  (params (Damage :type Float%20%28single-precision%29) (DamageType :type Damage%20Type%20Object%20Reference) (HitLocation :type Vector :default "0, 0, 0") (HitNormal :type Vector :default "0, 0, 0") (HitComponent :type Primitive%20Component%20Object%20Reference) (BoneName :type Name :default "None") (ShotFromDirection :type Vector :default "0, 0, 0") (InstigatedBy :type Controller%20Object%20Reference) (DamageCauser :type Actor%20Object%20Reference) (HitInfo :type Hit%20Result%20Structure%20%28by%20ref%29))
  (bind _hit_montage (Variables|Default|GetHit_Montage))
  ;[1 1 1] Got Damage
  (bind _returnvalue (UserInterface|CreateWidget "/Game/-RLS/Blueprints/Widgets/W_Hit.W_Hit_C"))
  (UserInterface|Viewport|AddtoViewport _returnvalue 0)
  (if (Utilities|Name|Equal(Name) BoneName "CATRigHub001Bone005Bone001")
    (Variables|Default|SetGotDamage false))
  (if (not (Variables|Default|GetGotDamage))
    (Variables|Default|SetGotDamage true)
    (if (Variables|/Game/-RLS/Blueprints/Components/BP_VitalityComponent.BP_VitalityComponent_C|GetIsAlive (Variables|Default|GetBP_VitalityComponent))
      (Animation|Montage|PlayMontage (Variables|Character|GetMesh) (Utilities|Array|Get(acopy) _hit_montage (Math|Random|RandomInteger (Utilities|Array|Length _hit_montage)))
        (:then
          (if (not (Variables|Default|GetIsHunting))
            (CallFunction|StartHunt)))))))

(event Game|Damage|EventAnyDamage
  (params (Damage :type Float%20%28single-precision%29) (DamageType :type Damage%20Type%20Object%20Reference) (InstigatedBy :type Controller%20Object%20Reference) (DamageCauser :type Actor%20Object%20Reference))
  (bind _hit_montage (Variables|Default|GetHit_Montage))
  ;[1 1 1] Got Damage
  (bind _returnvalue (UserInterface|CreateWidget "/Game/-RLS/Blueprints/Widgets/W_Hit.W_Hit_C"))
  (UserInterface|Viewport|AddtoViewport _returnvalue 0)
  (if (Utilities|Name|Equal(Name) (stale Game|Damage|EventPointDamage BoneName) "CATRigHub001Bone005Bone001")
    (Variables|Default|SetGotDamage false))
  (if (not (Variables|Default|GetGotDamage))
    (Variables|Default|SetGotDamage true)
    (if (Variables|/Game/-RLS/Blueprints/Components/BP_VitalityComponent.BP_VitalityComponent_C|GetIsAlive (Variables|Default|GetBP_VitalityComponent))
      (Animation|Montage|PlayMontage (Variables|Character|GetMesh) (Utilities|Array|Get(acopy) _hit_montage (Math|Random|RandomInteger (Utilities|Array|Length _hit_montage)))
        (:then
          (if (not (Variables|Default|GetIsHunting))
            (CallFunction|StartHunt)))))))

(event Game|Damage|EventRadialDamage
  (params (DamageReceived :type Float%20%28single-precision%29) (DamageType :type Damage%20Type%20Object%20Reference) (Origin :type Vector :default "0, 0, 0") (HitInfo :type Hit%20Result%20Structure%20%28by%20ref%29) (InstigatedBy :type Controller%20Object%20Reference) (DamageCauser :type Actor%20Object%20Reference))
  (bind _hit_montage (Variables|Default|GetHit_Montage))
  ;[1 1 1] Got Damage
  (bind _returnvalue (UserInterface|CreateWidget "/Game/-RLS/Blueprints/Widgets/W_Hit.W_Hit_C"))
  (UserInterface|Viewport|AddtoViewport _returnvalue 0)
  (if (Utilities|Name|Equal(Name) (stale Game|Damage|EventPointDamage BoneName) "CATRigHub001Bone005Bone001")
    (Variables|Default|SetGotDamage false))
  (if (not (Variables|Default|GetGotDamage))
    (Variables|Default|SetGotDamage true)
    (if (Variables|/Game/-RLS/Blueprints/Components/BP_VitalityComponent.BP_VitalityComponent_C|GetIsAlive (Variables|Default|GetBP_VitalityComponent))
      (Animation|Montage|PlayMontage (Variables|Character|GetMesh) (Utilities|Array|Get(acopy) _hit_montage (Math|Random|RandomInteger (Utilities|Array|Length _hit_montage)))
        (:then
          (if (not (Variables|Default|GetIsHunting))
            (CallFunction|StartHunt)))))))

(fn ConstructionScript)

(fn GetHPWidget
  (bind _asw_hp (Utilities|Casting|CastToW_HP (UserInterface|GetUserWidgetObject (Variables|Components|GetWidget_HP))))
  (return _asw_hp))

(fn SpawnWeaponLegs
  (bind _returnvalue (Game|SpawnActorfromClass "/Game/-RLS/Blueprints/Enemy/Weapon/BP_EW_ArachnidLeg.BP_EW_ArachnidLeg_C" (Math|Transform|MakeTransform "0, 0, 0" "0, 0, 0" "1,1,1") "AlwaysSpawn" 0 0))
  (Variables|Default|SetRightClaw _returnvalue)
  (bind _returnvalue_2 (Game|SpawnActorfromClass "/Game/-RLS/Blueprints/Enemy/Weapon/BP_EW_ArachnidLeg.BP_EW_ArachnidLeg_C" (Math|Transform|MakeTransform "0, 0, 0" "0, 0, 0" "1,1,1") "AlwaysSpawn" 0 0))
  (Variables|Default|SetLeftClaw _returnvalue_2)
  (bind _returnvalue_3 (Game|SpawnActorfromClass "/Game/-RLS/Blueprints/Enemy/Weapon/BP_EW_ArachnidLeg.BP_EW_ArachnidLeg_C" (Math|Transform|MakeTransform "0, 0, 0" "0, 0, 0" "1,1,1") "AlwaysSpawn" 0 0))
  (Variables|Default|SetRightLeg _returnvalue_3)
  (bind _returnvalue_4 (Game|SpawnActorfromClass "/Game/-RLS/Blueprints/Enemy/Weapon/BP_EW_ArachnidLeg.BP_EW_ArachnidLeg_C" (Math|Transform|MakeTransform "0, 0, 0" "0, 0, 0" "1,1,1") "AlwaysSpawn" 0 0))
  (Variables|Default|SetLeftLeg _returnvalue_4)
  (Transformation|AttachComponentToComponent (Variables|Default|GetRightClaw) (Variables|Character|GetMesh) "RightClaw" "SnapToTarget" "SnapToTarget" "SnapToTarget" true)
  (Transformation|AttachComponentToComponent (Variables|Default|GetLeftClaw) (Variables|Character|GetMesh) "LeftClaw" "SnapToTarget" "SnapToTarget" "SnapToTarget" true)
  (Transformation|AttachComponentToComponent (Variables|Default|GetRightLeg) (Variables|Character|GetMesh) "RightLeg" "SnapToTarget" "SnapToTarget" "SnapToTarget" true)
  (Transformation|AttachComponentToComponent (Variables|Default|GetLeftLeg) (Variables|Character|GetMesh) "LeftLeg" "KeepRelative" "KeepRelative" "KeepRelative" true))