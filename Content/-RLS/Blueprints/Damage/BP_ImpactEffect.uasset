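; BP_ImpactEffect is a short-lived actor that plays surface-specific impact feedback for a hit.
; InitIE switches on the hit's physical material surface type to pick a particle, sound and decal, with Grass having no sound.
; It spawns the particle and sound at its own location, attaches a temporary decal to the hit component oriented by the surface normal, then destroys itself.
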(event Custom|InitIE
  (params (Hit :type Hit%20Result%20Structure))
  (bind (_bblockinghit _binitialoverlap _time _distance _location _impactpoint _normal _impactnormal _physmat _hitactor _hitcomponent) (Collision|BreakHitResult Hit))
  (bind _returnvalue (Transformation|GetActorLocation))
  (Utilities|FlowControl|Sequence
    (:then_0
      (switch Utilities|FlowControl|Switch|SwitchonEPhysicalSurface (Variables|/Script/PhysicsCore.PhysicalMaterial|GetSurfaceType _physmat)
        (:SurfaceType1
          (Variables|Default|SetCurrentParticle "/Game/BallisticsVFX/Particles/Impacts/DynamicImpacts/Rock/Rock_impact_2_Dyn.Rock_impact_2_Dyn")
          (Variables|Default|SetCurrentSound "/Game/-RLS/Music/Sounds/Impacts/Rock_1_Cue.Rock_1_Cue")
          (Variables|Default|SetCurrentDecal "/Game/BallisticsVFX/Decals/Splashers/Decal_Shot.Decal_Shot"))
        (:SurfaceType2
          (Variables|Default|SetCurrentParticle "/Game/BallisticsVFX/Particles/Impacts/DynamicImpacts/Metal/Metal_impact_Dyn.Metal_impact_Dyn")
          (Variables|Default|SetCurrentSound "/Game/-RLS/Music/Sounds/Impacts/Metal_Light_1_Cue.Metal_Light_1_Cue")
          (Variables|Default|SetCurrentDecal "/Game/BallisticsVFX/Decals/Splashers/Decal_Shot.Decal_Shot"))
        (:SurfaceType3
          (Variables|Default|SetCurrentParticle "/Game/BallisticsVFX/Particles/Impacts/DynamicImpacts/Wood/Wood_impact_Dyn.Wood_impact_Dyn")
          (Variables|Default|SetCurrentSound "/Game/-RLS/Music/Sounds/Impacts/Wood_Light_1_Cue.Wood_Light_1_Cue")
          (Variables|Default|SetCurrentDecal "/Game/BallisticsVFX/Decals/Splashers/Decal_Shot.Decal_Shot"))
        (:SurfaceType4
          (Variables|Default|SetCurrentParticle "/Game/BallisticsVFX/Particles/Impacts/DynamicImpacts/Snow/Snow_impact_Dyn.Snow_impact_Dyn")
          (Variables|Default|SetCurrentSound "/Game/-RLS/Music/Sounds/Impacts/Snow_1_Cue.Snow_1_Cue")
          (Variables|Default|SetCurrentDecal "/Game/BallisticsVFX/Decals/Splashers/Decal_Shot.Decal_Shot"))
        (:SurfaceType5
          (Variables|Default|SetCurrentParticle "/Game/BallisticsVFX/Particles/Impacts/DynamicImpacts/Concrete/Concrete_impact_2_Dyn.Concrete_impact_2_Dyn")
          (Variables|Default|SetCurrentSound "/Game/BallisticsVFX/SFX/Impacts/Concrete/Concrete_01_Cue.Concrete_01_Cue")
          (Variables|Default|SetCurrentDecal "/Game/BallisticsVFX/Decals/Decals_Concrete.Decals_Concrete"))
        (:SurfaceType6
          (Variables|Default|SetCurrentParticle "/Game/BallisticsVFX/Particles/Impacts/DynamicImpacts/Gravel/Gravel_Debris.Gravel_Debris")
          (Variables|Default|SetCurrentSound "/Game/BallisticsVFX/SFX/Impacts/Gravel/08-Gravel_Cue.08-Gravel_Cue")
          (Variables|Default|SetCurrentDecal "/Game/BallisticsVFX/Decals/Splashers/Decal_Shot.Decal_Shot"))
        (:SurfaceType7
          (Variables|Default|SetCurrentParticle "/Game/BallisticsVFX/Particles/ImpactsVROptimal/DynamicImpacts/Water/Water_impact_Dyn.Water_impact_Dyn")
          (Variables|Default|SetCurrentSound "/Game/-RLS/Music/Sounds/Impacts/Water_2_Cue.Water_2_Cue")
          (Variables|Default|SetCurrentDecal "/Game/BallisticsVFX/Decals/Splashers/Decal_Water_Splatter.Decal_Water_Splatter"))
        (:SurfaceType8
          (Variables|Default|SetCurrentParticle "/Game/BallisticsVFX/Particles/Impacts/DynamicImpacts/Grass/Grass_impact_Dyn.Grass_impact_Dyn")
          (Variables|Default|SetCurrentSound 0)
          (Variables|Default|SetCurrentDecal "/Game/BallisticsVFX/Decals/Splashers/Decal_Mud_Splatter.Decal_Mud_Splatter"))
        (:SurfaceType9
          (Variables|Default|SetCurrentParticle "/Game/BallisticsVFX/Particles/Impacts/DynamicImpacts/Dirt/Dirt_impact_Dyn.Dirt_impact_Dyn")
          (Variables|Default|SetCurrentSound "/Game/BallisticsVFX/SFX/Impacts/Dirt/Dirt_4_Cue.Dirt_4_Cue")
          (Variables|Default|SetCurrentDecal "/Game/BallisticsVFX/Decals/Splashers/Decal_Mud_Splatter.Decal_Mud_Splatter"))))
    (:then_1
      (Effects|SpawnEmitteratLocation (Variables|Default|GetCurrentParticle) _returnvalue (Math|Conversions|RotationFromXVector _normal))
      (Audio|SpawnSoundatLocation (Variables|Default|GetCurrentSound) _returnvalue "0, 0, 0" 1.0 1.0 0.0 0 0)
      (Class|GameplayStatics|SpawnDecalAttached (Variables|Default|GetCurrentDecal) "2.000000,2.000000,2.000000" _hitcomponent "None" _returnvalue (Math|Conversions|RotationFromXVector _impactnormal) "KeepWorldPosition" 6.0)
      (Actor|DestroyActor))))

(fn ConstructionScript)