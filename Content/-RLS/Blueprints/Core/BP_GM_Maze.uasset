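; Maze game mode that builds a run of randomly chosen rooms at BeginPlay, then fades the camera in from black after a short delay.
; The first BP_LevelAnchor found sets the starting transform, and SpawnLevels loads RoomAmount level instances, picked from MazeRoomMap keys with repeats possible.
; Each room's map entry chains the next spawn point by adding its location offset unrotated and replacing the rotation.
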(event Custom|SetFirstAnchor
  (bind _outactors (Actor|GetAllActorsOfClass "/Game/-RLS/Blueprints/Environment/BP_LevelAnchor.BP_LevelAnchor_C"))
  (if (Utilities|Array|IsValidIndex _outactors)
    (Variables|Default|SetFirstSpawnTransform (Transformation|GetActorTransform (Utilities|Array|Get(acopy) _outactors)))))

(event Custom|SpawnNextRoom
  (bind _output_get (Variables|Default|SetCurrentSubLevel (CallFunction|GetNextRoomName)))
  (Class|LevelStreamingDynamic|LoadLevelInstance _output_get (.location (Variables|Default|GetFirstSpawnTransform)) (.rotation (Variables|Default|GetFirstSpawnTransform)))
  (Development|PrintString (Utilities|String|ToString(Integer) (Variables|Default|Getcurrent%20room%20number)))
  (Variables|Default|SetFirstSpawnTransform (Math|Transform|MakeTransform (+ (.Location (Math|Transform|BreakTransform (.Value (Utilities|Map|Find (Variables|Default|GetMazeRoomMap) _output_get)))) (.location (Variables|Default|GetFirstSpawnTransform))) (.Rotation (Math|Transform|BreakTransform (.Value (Utilities|Map|Find (Variables|Default|GetMazeRoomMap) _output_get)))) "1,1,1"))
  (Math|Integer|IncrementInt (Variables|Default|Getcurrent%20room%20number)))

(event EventBeginPlay
  (bind _returnvalue (Game|GetPlayerCameraManager 0))
  (|CallParentFunction)
  (CallFunction|SetFirstAnchor)
  (|Spawnlevels)
  (Class|PlayerCameraManager|SetManualCameraFade :self _returnvalue :InFadeAmount 1.0)
  (Utilities|FlowControl|Delay 2.0)
  (CameraFades|StartCameraFade :self _returnvalue :FromAlpha 1.0 :Duration 3.0 :bHoldWhenFinished true))

(fn ConstructionScript
  (|CallParentFunction))

(fn GetNextRoomName
  (Utilities|FlowControl|Sequence
    (:then_0
      (bind _keys (Utilities|Map|Keys (Variables|Default|GetMazeRoomMap)))
      (LocalVariables|SetLocal_LevelName (Utilities|Array|Get(acopy) _keys (Math|Random|RandomInteger (Utilities|Array|Length _keys)))))
    (:then_1
      (return (LocalVariables|GetLocal_LevelName)))))