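; BP_GM is the game mode Blueprint that restores the player character's state on BeginPlay after arrival by portal or teleport.
; It reads the travel type and saved data from BP_GI, the game instance.
; For portals, it finds the BP_Portal_Level with the matching ID and offsets saved camera yaw by that destination's yaw plus 90 degrees.
; Otherwise, for teleports, it briefly hides the character mesh.
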(event EventBeginPlay
  ;[0 0.02558 1 1 30] When the character is sent through the Portal, the "GMB" will adjust the rotation of the character's camera to maintain the previous rotation. When the character is sent by Teleportation, the "GMB" will set the Character's Mesh to be invisible for 1.6 seconds.
  (bind _asbp_gi (Utilities|Casting|CastToBP_GI (Game|GetGameInstance)))
  (bind _asbp_character (Utilities|Casting|CastToBP_Character (Game|GetPlayerCharacter 0)))
  (if (Variables|/Game/-RLS/Blueprints/Core/BP_GI.BP_GI_C|GetPortal _asbp_gi)
    (bind _outactors (Actor|GetAllActorsOfClass "/Game/-RLS/Blueprints/Environment/Portals/BP_Portal_Level.BP_Portal_Level_C"))
    (for _array_element _outactors
      (if (Utilities|Name|Equal(Name) (Variables|/Game/-RLS/Blueprints/Environment/Portals/BP_Portal_Level.BP_Portal_Level_C|GetPortal%20ID _array_element) (Variables|/Game/-RLS/Blueprints/Core/BP_GI.BP_GI_C|GetID _asbp_gi))
        (Pawn|SetControlRotation (Pawn|GetController _asbp_character) (Math|Rotator|MakeRotator (Variables|/Game/-RLS/Blueprints/Core/BP_GI.BP_GI_C|GetCanera%20Rotation%20X _asbp_gi) (Variables|/Game/-RLS/Blueprints/Core/BP_GI.BP_GI_C|GetCanera%20Rotation%20Y _asbp_gi) (+ (+ (.yaw (Transformation|GetWorldRotation (Variables|/Game/-RLS/Blueprints/Environment/Portals/BP_Portal_Level.BP_Portal_Level_C|GetDestination%20Location _array_element))) 9e+01) (Variables|/Game/-RLS/Blueprints/Core/BP_GI.BP_GI_C|GetCanera%20Rotation%20Z _asbp_gi))))))
    (elif (Variables|/Game/-RLS/Blueprints/Core/BP_GI.BP_GI_C|GetTeleport _asbp_gi)
      (Rendering|SetVisibility (Variables|/Script/Engine.Character|GetMesh _asbp_character) false false)
      (Utilities|FlowControl|Delay 1.6)
      (Rendering|SetVisibility (Variables|/Script/Engine.Character|GetMesh _asbp_character) true false))))

(fn ConstructionScript)