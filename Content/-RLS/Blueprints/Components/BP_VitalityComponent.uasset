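; Actor component that manages its owner's health, damage intake, death and optional regeneration.
; While active, it handles the owner's point and radial damage of BP_DamageType_Base types, multiplying headshots and scaling by a resistance map keyed on damage impact.
; Scaled hits above a small threshold lower clamped HP, fire change and death dispatchers, and restart a delayed looping regen timer.
; Regen heals a percentage of total HP until full, stopping on component deactivation.
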(event Custom|PointDamage
  (params (DamagedActor :type Actor%20Object%20Reference) (Damage :type Float%20%28single-precision%29) (InstigatedBy :type Controller%20Object%20Reference) (HitLocation :type Vector) (FHitComponent :type Primitive%20Component%20Object%20Reference) (BoneName :type Name) (ShotFromDirection :type Vector) (DamageType :type Damage%20Type%20Object%20Reference) (DamageCauser :type Actor%20Object%20Reference))
  (bind _returnvalue (Collision|MakeHitResult true false 0.0 0.0 HitLocation HitLocation "0,0,1" "0,0,1" 0 DamagedActor FHitComponent BoneName))
  (if (Components|Activation|IsActive)
    (bind _asbp_damage_type_base (Utilities|Casting|CastToBP_DamageType_Base DamageType))
    (if (Utilities|Name|Equal(Name) BoneName "head")
      (CallFunction|ApplyDamage (* 4 Damage) _asbp_damage_type_base _returnvalue)
      (else
        (CallFunction|ApplyDamage Damage _asbp_damage_type_base _returnvalue)))))

(event Custom|RadialDamage
  (params (DamagedActor :type Actor%20Object%20Reference) (Damage :type Float%20%28single-precision%29) (DamageType :type Damage%20Type%20Object%20Reference) (Origin :type Vector) (HitInfo :type Hit%20Result%20Structure) (InstigatedBy :type Controller%20Object%20Reference) (DamageCauser :type Actor%20Object%20Reference))
  (if (Components|Activation|IsActive)
    (bind _asbp_damage_type_base (Utilities|Casting|CastToBP_DamageType_Base DamageType))
    (CallFunction|ApplyDamage Damage _asbp_damage_type_base HitInfo)))

(event Custom|OnDeactivete
  (params (Component :type Actor%20Component%20Object%20Reference))
  (Utilities|Time|ClearandInvalidateTimerbyHandle (Variables|-Regen|GetRegen_TH)))

(event EventBeginPlay
  (bind _returnvalue (Components|GetOwner))
  (Variables|-HP|SetCurrentHP (Variables|-HP|GetTotalHP))
  (Utilities|FlowControl|Sequence
    (:then_0
      (EventDispatchers|BindEventtoOnTakePointDamage _returnvalue (delegate Custom|PointDamage))
      (EventDispatchers|BindEventtoOnTakeRadialDamage _returnvalue (delegate Custom|RadialDamage))
      (EventDispatchers|BindEventtoOnComponentDeactivated (delegate Custom|OnDeactivete)))
    (:then_1
      (Utilities|FlowControl|Delay 0.0)
      (Default|CallOnHeal (Variables|-HP|GetCurrentHP) (Variables|-HP|GetTotalHP)))))

(fn ApplyDamage
  (params (Damage :type Float%20%28single-precision%29) (DamageType :type BP%20Damage%20Type%20Base%20Object%20Reference) (Hit :type Hit%20Result%20Structure))
  (LocalVariables|SetLocal_Hit Hit)
  (bind _actualdamage (CallFunction|ApplyDamageType Damage DamageType))
  (if (> _actualdamage 1.0)
    (CallFunction|ResetRegen)
    (bind _output_get (Variables|-HP|SetCurrentHP (Math|Float|Clamp(Float) (- (Variables|-HP|GetCurrentHP) _actualdamage) 0.0 (Variables|-HP|GetTotalHP))))
    (Default|CallOnHPChange _output_get (Variables|-HP|GetTotalHP) (LocalVariables|GetLocal_Hit) false)
    ;[1 1 1] Death
    (if (<= (Variables|-HP|GetCurrentHP) 0.0)
      (Variables|-RuntimeVariable|SetIsAlive false)
      (Default|CallOnDeath (LocalVariables|GetLocal_Hit)))))

(fn ApplyDamageType
  (params (BaseDamage :type Float%20%28single-precision%29) (DamageType :type BP%20Damage%20Type%20Base%20Object%20Reference))
  (bind _damageimpact (Variables|/Game/-RLS/Blueprints/Damage/DamageType/BP_DamageType_Base.BP_DamageType_Base_C|GetDamageImpact DamageType))
  (bind _resistancemap (Variables|-HP|GetResistanceMap))
  (bind (_value _returnvalue) (Utilities|Map|Find _resistancemap _damageimpact))
  (if _returnvalue
    (return (* BaseDamage _value))
    (else
      (return BaseDamage))))

(fn ResetRegen
  (if (Variables|-Regen|GetCanRegenerate)
    (Utilities|Time|ClearandInvalidateTimerbyHandle (Variables|-Regen|GetRegen_TH))
    (bind _returnvalue (Utilities|Time|SetTimerbyFunctionName self "Apply Regen Heal" (/ 1.0 (Variables|-Regen|GetTickPerSecond)) true (Variables|-Regen|GetActivateDelay)))
    (Variables|-Regen|SetRegen_TH _returnvalue)))

(fn ApplyRegenHeal
  (bind _totalhp (Variables|-HP|GetTotalHP))
  (bind _output_get (Variables|-HP|SetCurrentHP (Math|Float|Clamp(Float) (+ (Variables|-HP|GetCurrentHP) (* (/ (Variables|-Regen|GetRegenPercentHPPerSecond) (Variables|-Regen|GetTickPerSecond)) 0.01 (Variables|-HP|GetTotalHP))) 0.0 _totalhp)))
  (Default|CallOnHeal _output_get _totalhp)
  (if (>= _output_get _totalhp)
    (Utilities|Time|ClearandInvalidateTimerbyHandle (Variables|-Regen|GetRegen_TH))))

(fn UpdateHP
  (params (CurrentHP :type Float%20%28single-precision%29) (TotalHP :type Float%20%28single-precision%29))
  (Default|CallOnHPChange :CurrentHP CurrentHP :TotalHP TotalHP :Heal true)
  (return))