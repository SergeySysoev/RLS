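; BP_TargetCheck_Component is an actor component that detects when the player camera comes near or leaves its owner.
; Tick, toggled by component activation, measures camera distance and fires catch and release events, using separate CatchDistance and ReleaseDistance thresholds with a lock flag.
; IsVisible combines the release range with a Camera-channel trace toward the camera that must hit the player's BP_Character.
; A similar debug trace in the event graph is disconnected, so locking depends on distance alone.
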(event Custom|OnDeactivate
  (params (Component :type Actor%20Component%20Object%20Reference))
  (Components|Tick|SetComponentTickEnabled false))

(event Custom|OnActivate
  (params (Component :type Actor%20Component%20Object%20Reference) (bReset :type Boolean))
  (Components|Tick|SetComponentTickEnabled true))

(event EventBeginPlay
  (Variables|Default|SetTargetComponent (Variables|/Script/Engine.PlayerCameraManager|GetTransformComponent (Game|GetPlayerCameraManager 0)))
  (EventDispatchers|BindEventtoOnComponentDeactivated (delegate Custom|OnDeactivate))
  (Components|Activation|BindEventtoOnComponentActivated (delegate Custom|OnActivate)))

(event EventTick
  (params (DeltaSeconds :type Float%20%28single-precision%29))
  (Variables|-Runtimevariables|SetDistanceToTarget (Math|Vector|VectorLength (- (Transformation|GetWorldLocation (Variables|Default|GetTargetComponent)) (Transformation|GetActorLocation (Components|GetOwner)))))
  (if (Variables|-Runtimevariables|GetIsTargetLock)
    (if (> (Variables|-Runtimevariables|GetDistanceToTarget) (Variables|-EditableVariable|GetRelease_Distance))
      (Variables|-Runtimevariables|SetIsTargetLock false)
      (Default|CallOnReleaseTarget))
    (elif (< (Variables|-Runtimevariables|GetDistanceToTarget) (Variables|-EditableVariable|GetCatch_Distance))
      (Variables|-Runtimevariables|SetIsTargetLock true)
      (Default|CallOnCatchTarget))))

(fn IsVisible
  (bind _outhit (Collision|LineTraceByChannel (Transformation|GetActorLocation (Components|GetOwner)) (Camera|GetCameraLocation (Game|GetPlayerCameraManager 0)) "TraceTypeQuery2" true 0 "None" true "(R=0.000000,G=0.040459,B=1.000000,A=1.000000)" "(R=1.000000,G=0.019670,B=0.790094,A=1.000000)"))
  (bind _asbp_character (Utilities|Casting|CastToBP_Character (Game|GetPlayerCharacter 0)))
  (return (and (<= (Variables|-Runtimevariables|GetDistanceToTarget) (Variables|-EditableVariable|GetRelease_Distance)) (== (.HitActor (Collision|BreakHitResult _outhit)) _asbp_character))))