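; Ammo component that tracks clip and reserve ammo for six weapon types, each in its own struct variable.
; SpendAmmo removes one round from the selected weapon's clip, while ApplyReload refills it using a clip size hard-coded per weapon.
; CalculateReload tops up the clip from the reserve, giving a partial refill when the reserve runs short.
; Both spending and reloading broadcast the updated struct through the OnAmmoChange dispatcher.
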(event EventBeginPlay)

(event EventTick
  (params (DeltaSeconds :type Float%20%28single-precision%29)))

(fn SpendAmmo
  (params (NewParam :type E_WeaponName%20Enum :default "NewEnumerator0"))
  (bind _ammo_m16 (Variables|Default|GetAmmo_M16))
  (bind _ammo_ak74 (Variables|Default|GetAmmo_AK74))
  (bind _ammo_shotgun (Variables|Default|GetAmmo_Shotgun))
  (bind _ammo_rl (Variables|Default|GetAmmo_RL))
  (bind _ammo_pistol (Variables|Default|GetAmmo_Pistol))
  (bind _ammo_dbshotgun (Variables|Default|GetAmmo_DBShotgun))
  (Utilities|FlowControl|Sequence
    (:then_0
      (switch Utilities|FlowControl|Switch|SwitchonE_WeaponName NewParam
        (:NewEnumerator0
          (bind _structout (Utilities|Struct|SetmembersinStruct_WeaponAmmo _ammo_m16 (- (Utilities|Struct|BreakStruct_WeaponAmmo _ammo_m16) 1)))
          (Default|CallOnAmmoChange _structout))
        (:NewEnumerator1
          (bind _structout_2 (Utilities|Struct|SetmembersinStruct_WeaponAmmo _ammo_ak74 (- (Utilities|Struct|BreakStruct_WeaponAmmo _ammo_ak74) 1)))
          (Default|CallOnAmmoChange _structout_2))
        (:NewEnumerator2
          (bind _structout_3 (Utilities|Struct|SetmembersinStruct_WeaponAmmo _ammo_shotgun (- (Utilities|Struct|BreakStruct_WeaponAmmo _ammo_shotgun) 1)))
          (Default|CallOnAmmoChange _structout_3))
        (:NewEnumerator3
          (bind _structout_4 (Utilities|Struct|SetmembersinStruct_WeaponAmmo _ammo_rl (- (Utilities|Struct|BreakStruct_WeaponAmmo _ammo_rl) 1)))
          (Default|CallOnAmmoChange _structout_4))
        (:NewEnumerator4
          (bind _structout_5 (Utilities|Struct|SetmembersinStruct_WeaponAmmo _ammo_pistol (- (.InClip (Utilities|Struct|BreakStruct_WeaponAmmo _ammo_pistol)) 1)))
          (Default|CallOnAmmoChange _structout_5))
        (:NewEnumerator5
          (bind _structout_6 (Utilities|Struct|SetmembersinStruct_WeaponAmmo _ammo_dbshotgun (- (.InClip (Utilities|Struct|BreakStruct_WeaponAmmo _ammo_dbshotgun)) 1)))
          (Default|CallOnAmmoChange _structout_6))))))

(fn ApplyReload
  (params (NewParam :type E_WeaponName%20Enum :default "NewEnumerator0"))
  (bind _ammo_m16 (Variables|Default|GetAmmo_M16))
  (bind _ammo_ak74 (Variables|Default|GetAmmo_AK74))
  (bind _ammo_shotgun (Variables|Default|GetAmmo_Shotgun))
  (bind _ammo_rl (Variables|Default|GetAmmo_RL))
  (bind _ammo_pistol (Variables|Default|GetAmmo_Pistol))
  (bind _ammo_dbshotgun (Variables|Default|GetAmmo_DBShotgun))
  (bind (_inclip _total) (CallFunction|CalculateReload _ammo_rl 1))
  (bind (_inclip_2 _total_2) (CallFunction|CalculateReload _ammo_m16 8))
  (bind (_inclip_3 _total_3) (CallFunction|CalculateReload _ammo_ak74 30))
  (bind (_inclip_4 _total_4) (CallFunction|CalculateReload _ammo_shotgun 6))
  (bind (_inclip_5 _total_5) (CallFunction|CalculateReload _ammo_pistol 7))
  (bind (_inclip_6 _total_6) (CallFunction|CalculateReload _ammo_dbshotgun 2))
  (switch Utilities|FlowControl|Switch|SwitchonE_WeaponName NewParam
    (:NewEnumerator0
      (bind _structout (Utilities|Struct|SetmembersinStruct_WeaponAmmo _ammo_m16 _inclip_2 _total_2))
      (Default|CallOnAmmoChange _structout))
    (:NewEnumerator1
      (bind _structout_2 (Utilities|Struct|SetmembersinStruct_WeaponAmmo _ammo_ak74 _inclip_3 _total_3))
      (Default|CallOnAmmoChange _structout_2))
    (:NewEnumerator2
      (bind _structout_3 (Utilities|Struct|SetmembersinStruct_WeaponAmmo _ammo_shotgun _inclip_4 _total_4))
      (Default|CallOnAmmoChange _structout_3))
    (:NewEnumerator3
      (bind _structout_4 (Utilities|Struct|SetmembersinStruct_WeaponAmmo _ammo_rl _inclip _total))
      (Default|CallOnAmmoChange _structout_4))
    (:NewEnumerator4
      (bind _structout_5 (Utilities|Struct|SetmembersinStruct_WeaponAmmo _ammo_pistol _inclip_5 _total_5))
      (Default|CallOnAmmoChange _structout_5))
    (:NewEnumerator5
      (bind _structout_6 (Utilities|Struct|SetmembersinStruct_WeaponAmmo _ammo_dbshotgun _inclip_6 _total_6))
      (Default|CallOnAmmoChange _structout_6))))

(fn CalculateReload
  (params (Struct_WeaponAmmo :type Struct%20Weapon%20Ammo%20Structure%20%28by%20ref%29) (ClipSize :type Integer))
  (bind (_inclip _total) (Utilities|Struct|BreakStruct_WeaponAmmo Struct_WeaponAmmo))
  (Utilities|FlowControl|Sequence
    (:then_0
      (if (>= _total ClipSize)
        (LocalVariables|SetLocal_Clip ClipSize :!label _label)
        (LocalVariables|SetLocal_Total (- _total (- ClipSize _inclip)))
        (elif (> (- ClipSize _inclip) _total)
          (LocalVariables|SetLocal_Clip (+ _inclip _total))
          (LocalVariables|SetLocal_Total 0)
          (else
            (goto _label)))))
    (:then_1
      (return (LocalVariables|GetLocal_Clip) (LocalVariables|GetLocal_Total)))))